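; Game mode for the EyeContact end map that handles team-based spawning and provides a reset of match status.
; ChoosePlayerStart gets the player's team from the controller and uses a random position from the first BP_EyeContactPlayerStart of that type.
; It falls back to the first such start, or to the first PlayerStart when the controller cast fails.
; ResetGameStatus marks the game ongoing and clears the human and monster player lists in GameState and GameInstance.
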(event EventBeginPlay)

(event EventTick
  (params (DeltaSeconds :type Float%20%28single-precision%29)))

(fn ConstructionScript)

(fn ResetGameStatus
  (bind _asbp_eye_contact_game_state (Utilities|Casting|CastToBP_EyeContactGameState (Game|GetGameState)))
  (Variables|/Game/EyeContact/Blueprints/BP_EyeContactGameState.BP_EyeContactGameState_C|SetGameIsOngoing _asbp_eye_contact_game_state true)
  (Utilities|Array|Clear (Variables|/Game/EyeContact/Blueprints/BP_EyeContactGameState.BP_EyeContactGameState_C|GetMonsterPlayers _asbp_eye_contact_game_state))
  (bind _asbp_eye_contact_game_instance (Utilities|Casting|CastToBP_EyeContactGameInstance (Game|GetGameInstance)))
  (Utilities|Array|Clear (Variables|/Game/EyeContact/Blueprints/BP_EyeContactGameInstance.BP_EyeContactGameInstance_C|GetHumanPlayerIds _asbp_eye_contact_game_instance))
  (Utilities|Array|Clear (Variables|/Game/EyeContact/Blueprints/BP_EyeContactGameInstance.BP_EyeContactGameInstance_C|GetMonsterPlayerIds _asbp_eye_contact_game_instance)))

(fn ChoosePlayerStart
  (params (Player :type Controller%20Object%20Reference))
  (bind _asbp_eye_contact_controller (Utilities|Casting|CastToBP_EyeContactController Player)
    (:then
      (bind _selectiontype (Default|GetPlayerTeam _asbp_eye_contact_controller (Variables|/Script/Engine.PlayerState|GetPlayerId (Variables|/Script/Engine.Controller|GetPlayerState Player))))
      (bind _outactors (Actor|GetAllActorsOfClass "/Game/EyeContact/Blueprints/BP_EyeContactPlayerStart.BP_EyeContactPlayerStart_C"))
      (for _array_element _outactors
        (if (Utilities|Enum|Equal(Enum) _selectiontype (Variables|/Game/EyeContact/Blueprints/BP_EyeContactPlayerStart.BP_EyeContactPlayerStart_C|GetPlayerType _array_element))
          (bind _spawnposition (Default|GetRandomSpawnPosition _array_element))
          (return _spawnposition)))
      (bind _spawnposition_2 (Default|GetRandomSpawnPosition (Utilities|Array|Get(acopy) _outactors)))
      (return _spawnposition_2))
    (:CastFailed
      ;[1 1 1] No BP_EyeContactPlayerStart found
      (bind _outactors_2 (Actor|GetAllActorsOfClass "/Script/Engine.PlayerStart"))
      (return (Utilities|Array|Get(acopy) _outactors_2)))))