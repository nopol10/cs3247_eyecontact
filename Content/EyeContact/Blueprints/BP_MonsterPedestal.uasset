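; BP_MonsterPedestal is a pedestal actor that may spawn a random actor from its PossibleActors list when play begins.
; On BeginPlay, only the authority rolls a random float against SpawnChance to decide whether to call SpawnRandomMesh.
; Despite its name, SpawnRandomMesh spawns a whole actor of a randomly picked class at the SpawnPoint component's world transform.
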(event EventBeginPlay
  (Networking|SwitchHasAuthority
    (:Authority
      (if (>= (Variables|Default|GetSpawnChance) (Math|Random|RandomFloat))
        (CallFunction|SpawnRandomMesh)))))

(event EventActorBeginOverlap
  (params (OtherActor :type Actor%20Object%20Reference)))

(event EventTick
  (params (DeltaSeconds :type Float%20%28single-precision%29)))

(fn ConstructionScript)

(fn SpawnRandomMesh
  (bind _possibleactors (Variables|Default|GetPossibleActors))
  (Game|SpawnActorfromClass (Utilities|Array|Get(acopy) _possibleactors (Math|Random|RandomIntegerinRange 0 (Utilities|Array|LastIndex _possibleactors))) (Transformation|GetWorldTransform (Variables|Default|GetSpawnPoint)) "Undefined" 0 0))