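; BP_Ice_Floor is an ice floor piece that randomizes its own look when play begins.
; It gives its static mesh one of three snowy rock or terrain materials at random.
; All branches then share one path that randomizes the mesh's vertical scale and snaps its world rotation to a random quarter turn, adding variation between pieces.
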(event EventBeginPlay
  (bind _staticmesh (Variables|Default|GetStaticMesh))
  (switch int (Math|Random|RandomIntegerinRange 0 2)
    (:0
      (Rendering|Material|SetMaterial _staticmesh 0 "/Game/InfinityBladeIceLands/Environments/Ice/DR_Ice_Mountain/Materials/M_Snowy_Rocky_Terrain.M_Snowy_Rocky_Terrain"))
    (:1
      (Rendering|Material|SetMaterial _staticmesh 0 "/Game/InfinityBladeIceLands/Environments/Ice/Env_Ice_MountainPaths/Materials/M_Snowy_Rocky_Ground.M_Snowy_Rocky_Ground"))
    (:2
      (Rendering|Material|SetMaterial _staticmesh 0 "/Game/InfinityBladeIceLands/Environments/Ice/DR_Ice_Mountain/Materials/M_Snowy_Rock_Slope.M_Snowy_Rock_Slope")))
  (Transformation|SetWorldScale3D _staticmesh (Math|Vector|MakeVector 1.0 1.0 (Math|Random|RandomFloatinRange 0.1 0.5)))
  (switch int (Math|Random|RandomIntegerinRange 0 3)
    (:0
      (Transformation|SetWorldRotation _staticmesh "0, 0, 0" false false))
    (:1
      (Transformation|SetWorldRotation _staticmesh "0,90.000000, 0" false false))
    (:2
      (Transformation|SetWorldRotation _staticmesh "0,180.000000, 0" false false))
    (:3
      (Transformation|SetWorldRotation _staticmesh "0,270.000000, 0" false false))))

(event Collision|EventActorBeginOverlap
  (params (OtherActor :type Actor%20Object%20Reference)))

(event EventTick
  (params (DeltaSeconds :type Float%20%28single-precision%29)))

(fn ConstructionScript)