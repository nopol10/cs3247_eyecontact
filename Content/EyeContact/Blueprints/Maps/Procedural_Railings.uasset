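; Procedural railing actor that builds a row of pillars toward an EndPoint offset when constructed in the level.
; The construction script derives the pillar count from the EndPoint distance and attaches thin, scaled static mesh components at even steps along the root StaticMesh's local X axis.
; It then yaws StaticMesh toward EndPoint, so the whole row follows that direction horizontally; the event graph has no active logic.
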(event EventBeginPlay)

(event EventActorBeginOverlap
  (params (OtherActor :type Actor%20Object%20Reference)))

(event EventTick
  (params (DeltaSeconds :type Float%20%28single-precision%29)))

(fn ConstructionScript
  (bind _returnvalue (Transformation|GetActorLocation))
  (if (Math|Vector|NotEqual(Vector) (+ (Variables|Default|GetEndPoint) "1.000000,1.000000, 0") "0, 0, 0" 0.0001)
    (for _index (range 1 (Math|Float|Floor (/ (Math|Vector|VectorLength (Variables|Default|GetEndPoint)) 5e+01)))
      ;[1 1 1] Create new pillar based on distance
      (bind _returnvalue_2 (AddComponent|AddStaticMeshComponent true (Math|Transform|MakeTransform "0, 0, 0" "0, 0, 0" "0.100000,0.100000,1.200000")))
      (Class|SceneComponent|Attachto _returnvalue_2 (Variables|Default|GetStaticMesh) "None" "KeepWorldPosition" true)
      (Transformation|SetRelativeLocation _returnvalue_2 (Math|Vector|MakeVector (* _index 5e+02) 0.0 0.0) false false))
    (Transformation|SetWorldRotation (Variables|Default|GetStaticMesh) (Math|Rotator|MakeRotator 0.0 0.0 (.Yaw (Math|Rotator|BreakRotator (Math|Rotator|FindLookatRotation _returnvalue (+ _returnvalue (Variables|Default|GetEndPoint)))))) false false)))