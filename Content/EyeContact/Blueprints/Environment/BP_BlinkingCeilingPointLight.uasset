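; Networked ceiling point light that flickers and controls whether co-op monsters beneath it can be seen.
; The server loops timed blinks and an off period, replicating ShouldOnLight through a RepNotify that toggles the light.
; Monsters inside DarkZone have CanBeSeen follow the light state, restored on exit.
; A human player entering KillLightZone marks the light dead, keeping it dark and ending the loop after the current cycle.
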(event OnComponentBeginOverlap(DarkZone)
  (params (OverlappedComponent :type Primitive%20Component%20Object%20Reference) (OtherActor :type Actor%20Object%20Reference) (OtherComp :type Primitive%20Component%20Object%20Reference) (OtherBodyIndex :type Integer) (bFromSweep :type Boolean) (SweepResult :type Hit%20Result%20Structure%20%28by%20ref%29))
  (Networking|SwitchHasAuthority
    (:Authority
      (bind _asbp_monster_coop (Utilities|Casting|CastToBP_MonsterCoop OtherActor))
      (Utilities|Array|AddUnique (Variables|Default|GetInZoneMonsters) _asbp_monster_coop)
      (Variables|/Game/EyeContact/Blueprints/BP_MonsterCoop.BP_MonsterCoop_C|SetCanBeSeen _asbp_monster_coop (Variables|Default|GetShouldOnLight)))))

(event OnComponentEndOverlap(DarkZone)
  (params (OverlappedComponent :type Primitive%20Component%20Object%20Reference) (OtherActor :type Actor%20Object%20Reference) (OtherComp :type Primitive%20Component%20Object%20Reference) (OtherBodyIndex :type Integer))
  (Networking|SwitchHasAuthority
    (:Authority
      (bind _asbp_monster_coop (Utilities|Casting|CastToBP_MonsterCoop OtherActor))
      (Utilities|Array|RemoveItem (Variables|Default|GetInZoneMonsters) _asbp_monster_coop)
      (Variables|/Game/EyeContact/Blueprints/BP_MonsterCoop.BP_MonsterCoop_C|SetCanBeSeen _asbp_monster_coop true))))

(event OnComponentBeginOverlap(KillLightZone)
  (params (OverlappedComponent :type Primitive%20Component%20Object%20Reference) (OtherActor :type Actor%20Object%20Reference) (OtherComp :type Primitive%20Component%20Object%20Reference) (OtherBodyIndex :type Integer) (bFromSweep :type Boolean) (SweepResult :type Hit%20Result%20Structure%20%28by%20ref%29))
  (Utilities|Casting|CastToHumanPlayer OtherActor)
  (CallFunction|ServerKillLight))

(event Custom|IntervalBlink
  (Utilities|FlowControl|Delay (Variables|Default|GetBlinkInterval))
  (CallFunction|IntervalReachedBlink))

(event Custom|IntervalOff
  (Utilities|FlowControl|Delay (Variables|Default|GetOffInterval))
  (CallFunction|IntervalReachedOff))

(event Custom|IntervalReachedOff
  (Variables|Default|SetShouldOnLight false)
  (Utilities|FlowControl|Delay (Variables|Default|GetOffDuration))
  (Variables|Default|SetShouldOnLight true)
  (if (not (Variables|Default|GetIsDeadLight))
    (CallFunction|IntervalBlink)))

(event Custom|IntervalReachedBlink
  (bind _blinkduration (Variables|Default|GetBlinkDuration))
  (Variables|Default|SetShouldOnLight false)
  (Utilities|FlowControl|Delay _blinkduration)
  (Variables|Default|SetShouldOnLight true)
  (Utilities|FlowControl|Delay _blinkduration)
  (Variables|Default|SetShouldOnLight false)
  (Utilities|FlowControl|Delay _blinkduration)
  (Variables|Default|SetShouldOnLight true)
  (CallFunction|IntervalOff))

(event Custom|ServerKillLight
  (Networking|SwitchHasAuthority
    (:Authority
      (Variables|Default|SetIsDeadLight true)
      (Variables|Default|SetShouldOnLight false))))

(event EventBeginPlay
  (Networking|SwitchHasAuthority
    (:Authority
      (CallFunction|IntervalBlink))))

(fn ConstructionScript)

(fn GenerateNextOffDuration
  (Variables|Default|SetOffDuration (Math|Random|RandomFloatinRange 0.2 0.7))
  (Variables|Default|SetOffTimer (Math|Random|RandomFloatinRange 0.2 5.0))
  (return))

(fn UpdateOffTimer
  (params (deltaTime :type Float%20%28single-precision%29))
  (if (<= (Variables|Default|GetOffTimer) 0.0)
    (bind _output_get (Variables|Default|SetOffDuration (- (Variables|Default|GetOffDuration) deltaTime)))
    (if (<= _output_get 0.0)
      (CallFunction|ToggleLight true)
      (CallFunction|GenerateNextOffDuration))
    (return)
    (else
      (bind _output_get_2 (Variables|Default|SetOffTimer (- (Variables|Default|GetOffTimer) deltaTime)))
      (if (<= _output_get_2 0.0)
        (CallFunction|ToggleLight false)
        (return)))))

(fn ToggleLight
  (params (shouldLightOn :type Boolean))
  (Rendering|SetVisibility (Variables|Default|GetPointLight) shouldLightOn false)
  (return))

(fn OnRepShouldonLight
  (if (Variables|Default|GetIsDeadLight)
    (CallFunction|ToggleLight false)
    (else
      (CallFunction|ToggleLight (Variables|Default|GetShouldOnLight))))
  (Networking|SwitchHasAuthority
    (:Authority
      (for _array_element (Variables|Default|GetInZoneMonsters)
        (Variables|/Game/EyeContact/Blueprints/BP_MonsterCoop.BP_MonsterCoop_C|SetCanBeSeen _array_element (Variables|Default|GetShouldOnLight))))))