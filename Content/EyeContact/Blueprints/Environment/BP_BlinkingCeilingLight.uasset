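; A ceiling light actor that flickers at random intervals by briefly switching its spot light off.
; Each tick, a countdown runs while the light is on, then hides the SpotLight component when it expires.
; A second, shorter countdown then restores visibility and rolls new random on and off durations, so the blink never follows a fixed rhythm.
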(event EventBeginPlay
  (CallFunction|GenerateNextOffDuration))

(event Collision|EventActorBeginOverlap
  (params (OtherActor :type Actor%20Object%20Reference)))

(event EventTick
  (params (DeltaSeconds :type Float%20%28single-precision%29))
  (CallFunction|UpdateOffTimer DeltaSeconds))

(fn ConstructionScript)

(fn GenerateNextOffDuration
  (Variables|Default|SetOffDuration (Math|Random|RandomFloatinRange 0.2 0.7))
  (Variables|Default|SetOffTimer (Math|Random|RandomFloatinRange 0.2 5.0))
  (return))

(fn UpdateOffTimer
  (params (deltaTime :type Float%20%28single-precision%29))
  (if (<= (Variables|Default|GetOffTimer) 0.0)
    (bind _output_get (Variables|Default|SetOffDuration (- (Variables|Default|GetOffDuration) deltaTime)))
    (if (<= _output_get 0.0)
      (CallFunction|ToggleLight true)
      (CallFunction|GenerateNextOffDuration))
    (return)
    (else
      (bind _output_get_2 (Variables|Default|SetOffTimer (- (Variables|Default|GetOffTimer) deltaTime)))
      (if (<= _output_get_2 0.0)
        (CallFunction|ToggleLight false)
        (return)))))

(fn ToggleLight
  (params (shouldLightOn :type Boolean))
  (Rendering|SetVisibility (Variables|Default|GetSpotLight) shouldLightOn false)
  (return))