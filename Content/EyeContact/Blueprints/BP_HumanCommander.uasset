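; Human commander player that watches the level from CCTV camera positions, with its mesh scaled to zero and movement disabled.
; On BeginPlay it clears goal info, finds the first BP_CCTVs actor, storing it only on authority, and moves to the current camera.
; MenuLeft and MenuRight cycle cameras through that manager.
; PossessCamera only teleports the actor to the camera's location, without changing possession or rotation.
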(event Custom|PossessCamera
  (params (Actor :type Camera%20Actor%20Object%20Reference))
  (Transformation|SetActorLocation (Transformation|GetActorLocation Actor) false true))

(event EventBeginPlay
  (|CallParentFunction)
  (Variables|Default|SetShouldEnableMovement false)
  (Transformation|SetWorldScale3D (Variables|Character|GetMesh) "0, 0, 0")
  (CallFunction|DeleteGoalInfo)
  (bind _outactors (Actor|GetAllActorsOfClass "/Game/EyeContact/Blueprints/BP_CCTVs.BP_CCTVs_C"))
  (if (> (Utilities|Array|Length _outactors) 0)
    (Networking|SwitchHasAuthority
      (:Authority
        (bind _output_get (Variables|Default|SetCCTVs (Utilities|Array|Get(acopy) _outactors))))
      (:Remote
        _))
    (bind _currentcctv (Default|GetCurrentCCTV _output_get))
    (CallFunction|PossessCamera _currentcctv)
    (Development|PrintString (Utilities|String|ToString(Integer) (Utilities|Array|Length (Variables|/Game/EyeContact/Blueprints/BP_CCTVs.BP_CCTVs_C|GetCCTVs _output_get))) true true "(R=0.258146,G=1.000000,B=0.528215,A=1.000000)" 3e+01)
    (else
      (Development|PrintString "NO CCTVS FOUND!"))))

(event Collision|EventActorBeginOverlap
  (params (OtherActor :type Actor%20Object%20Reference)))

(event EventTick
  (params (DeltaSeconds :type Float%20%28single-precision%29))
  (for _index (range 0 1)
    _))

(event Input|ActionEvents|InputActionMenuLeft
  (params (Key :type Key%20Structure :default "AnyKey"))
  (:Pressed
    (bind _prevcctv (Default|GetPrevCCTV (Variables|Default|GetCCTVs)))
    (CallFunction|PossessCamera _prevcctv)))

(event Input|ActionEvents|InputActionMenuRight
  (params (Key :type Key%20Structure :default "AnyKey"))
  (:Pressed
    (bind _nextcctv (Default|GetNextCCTV (Variables|Default|GetCCTVs)))
    (CallFunction|PossessCamera _nextcctv)))

(fn ConstructionScript
  (|CallParentFunction))