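; Lobby actor that shows the join-game browser as a 3D world widget.
; It starts at zero scale and binds the browser's close events on BeginPlay.
; EnableWidget timeline-scales it up with UI-only input; closing scales it down and restores game-only input.
; OpenTeamSelectMenu spawns an offset team-select 3D widget and returns its waiting-for-player dialog.
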(event Custom|EnableWidget
  (if (not (Variables|Default|GetIsShowingJoin))
    (Variables|Default|SetIsShowingJoin true)
    (Input|SetInputModeUIOnly (Game|GetPlayerController 0) (UserInterface|GetUserWidgetObject (Variables|Default|GetJoinMenu)) false)
    (bind _uppy (Timeline|ScaleUpWidget PlayFromStart)
      (:Update
        (Transformation|SetActorScale3D (Math|Vector|MakeVector _uppy _uppy _uppy))))))

(event Custom|CloseWidget
  (bind _returnvalue (Game|GetPlayerController 0))
  (bind _uppy (Timeline|ScaleDown PlayFromStart)
    (:Update
      (Transformation|SetActorScale3D (Math|Vector|MakeVector _uppy _uppy _uppy))
      (Variables|/Script/Engine.PlayerController|SetbShowMouseCursor _returnvalue false)
      (Input|SetInputModeGameOnly _returnvalue))
    (:Finished
      (Variables|Default|SetIsShowingJoin false))))

(event EventBeginPlay
  (Utilities|FlowControl|Sequence
    (:then_0
      (Variables|/Script/Engine.PlayerController|SetbShowMouseCursor (Game|GetPlayerController 0) false)
      (CallFunction|FaceObject (VehicleSound|GetRootComponent (Pawn|GetControlledPawn (Game|GetPlayerController 0))) self))
    (:then_1
      (Transformation|SetActorScale3D "0, 0, 0"))
    (:then_2
      (bind _asw_join_game_browser (Utilities|Casting|CastToW_JoinGameBrowser (UserInterface|GetUserWidgetObject (Variables|Default|GetJoinMenu))))
      (EventDispatchers|BindEventtoOnClicked (Variables|/Game/EyeContact/Interface/W_JoinGameBrowser.W_JoinGameBrowser_C|GetClose _asw_join_game_browser) (delegate Custom|CloseWidget))
      (EventDispatchers|BindEventtoOnCloseButtonPressed _asw_join_game_browser (delegate Custom|CloseWidget)))))

(event Collision|EventActorBeginOverlap
  (params (OtherActor :type Actor%20Object%20Reference)))

(event EventTick
  (params (DeltaSeconds :type Float%20%28single-precision%29)))

(fn ConstructionScript)

(fn OpenTeamSelectMenu
  (bind _returnvalue (Transformation|GetActorTransform))
  (bind _returnvalue_2 (Game|SpawnActorfromClass "/Game/EyeContact/Blueprints/TeamSelect/BP_SelectTeamWidget3D.BP_SelectTeamWidget3D_C" (Math|Transform|MakeTransform (Math|Vector|MakeVector (+ (.x (.location _returnvalue)) 3e+02) (.y (.location _returnvalue)) (.z (.location _returnvalue))) (.rotation _returnvalue) (.scale _returnvalue)) "Undefined" (Game|GetPlayerController 0) 0))
  (bind _asw_waiting_for_player_dialog (Utilities|Casting|CastToW_WaitingForPlayerDialog (UserInterface|GetUserWidgetObject (Variables|/Game/EyeContact/Blueprints/TeamSelect/BP_SelectTeamWidget3D.BP_SelectTeamWidget3D_C|GetLobbyMenu _returnvalue_2)))
    (:then
      (return _asw_waiting_for_player_dialog))
    (:CastFailed
      (return 0))))