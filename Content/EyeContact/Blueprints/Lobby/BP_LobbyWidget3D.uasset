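; BP_LobbyWidget3D is an in-world lobby menu actor that hosts its UI in a LobbyMenu widget component.
; On BeginPlay it switches the player to UI-only input focused on that widget, shows the cursor and calls FaceObject between the pawn's root and itself.
; OpenTeamSelectMenu spawns a BP_SelectTeamWidget3D offset along world X, owned by the player controller, and returns its widget cast to W_WaitingForPlayerDialog.
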(event EventBeginPlay
  (bind _returnvalue (Game|GetPlayerController 0))
  (Input|SetInputModeUIOnly _returnvalue (UserInterface|GetUserWidgetObject (Variables|Default|GetLobbyMenu)) false)
  (Variables|/Script/Engine.PlayerController|SetbShowMouseCursor _returnvalue true)
  (CallFunction|FaceObject (VehicleSound|GetRootComponent (Pawn|GetControlledPawn (Game|GetPlayerController 0))) self))

(event EventActorBeginOverlap
  (params (OtherActor :type Actor%20Object%20Reference)))

(event EventTick
  (params (DeltaSeconds :type Float%20%28single-precision%29)))

(fn ConstructionScript)

(fn OpenTeamSelectMenu
  (bind _returnvalue (Transformation|GetActorTransform))
  (bind _returnvalue_2 (Game|SpawnActorfromClass "/Game/EyeContact/Blueprints/TeamSelect/BP_SelectTeamWidget3D.BP_SelectTeamWidget3D_C" (Math|Transform|MakeTransform (Math|Vector|MakeVector (+ (.x (.location _returnvalue)) 3e+02) (.y (.location _returnvalue)) (.z (.location _returnvalue))) (.rotation _returnvalue) (.scale _returnvalue)) "Undefined" (Game|GetPlayerController 0) 0))
  (bind _asw_waiting_for_player_dialog (Utilities|Casting|CastToW_WaitingForPlayerDialog (UserInterface|GetUserWidgetObject (Variables|/Game/EyeContact/Blueprints/TeamSelect/BP_SelectTeamWidget3D.BP_SelectTeamWidget3D_C|GetLobbyMenu _returnvalue_2)))
    (:then
      (return _asw_waiting_for_player_dialog))
    (:CastFailed
      (return 0))))