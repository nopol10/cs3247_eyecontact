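; BP_MonsterIllusion is a spawner that creates an illusion matching the instigating BP_MonsterPlayer's current model.
; On BeginPlay, the server picks a class from PossibleActors by CurrentModelEnum and spawns it at SpawnPoint with randomized yaw.
; When the illusion is destroyed, it destroys the spawned actor too.
; Despite the SpawnRandomMesh name, only yaw is random, and the SpawnChance roll is disconnected.
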(event Custom|OnDestroyed_Event_0
  (params (DestroyedActor :type Actor%20Object%20Reference))
  (Actor|DestroyActor (Variables|Default|Getactor)))

(event EventBeginPlay
  (Networking|SwitchHasAuthority
    (:Authority
      (CallFunction|SpawnRandomMesh)
      (EventDispatchers|AssignOnDestroyed (delegate Custom|OnDestroyed_Event_0)))))

(event Collision|EventActorBeginOverlap
  (params (OtherActor :type Actor%20Object%20Reference)))

(event EventTick
  (params (DeltaSeconds :type Float%20%28single-precision%29)))

(fn ConstructionScript)

(fn SpawnRandomMesh
  (bind _spawnpoint (Variables|Default|GetSpawnPoint))
  (bind _returnvalue (Transformation|GetWorldRotation _spawnpoint))
  (bind _asbp_monster_player (Utilities|Casting|CastToBP_MonsterPlayer (Game|GetInstigator)))
  (bind _returnvalue_2 (Game|SpawnActorfromClass (Utilities|Array|Get(acopy) (Variables|Default|GetPossibleActors) (Math|Conversions|ToInteger(Byte) (Variables|/Game/EyeContact/Blueprints/BP_MonsterPlayer.BP_MonsterPlayer_C|GetCurrentModelEnum _asbp_monster_player))) (Math|Transform|MakeTransform (Transformation|GetWorldLocation _spawnpoint) (Math|Rotator|MakeRotator (.roll _returnvalue) (.pitch _returnvalue) (+ (.yaw _returnvalue) (Math|Random|RandomFloatinRange 0.0 3.6e+02))) (Transformation|GetWorldScale _spawnpoint)) "Undefined" 0 0))
  (Variables|Default|Setactor _returnvalue_2))