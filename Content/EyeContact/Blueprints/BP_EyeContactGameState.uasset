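; Game state for the EyeContact game that randomizes the level layout on the server at BeginPlay.
; It keeps one random end goal as active and replaces the others with exit blockers, then updates all direction signs and keeps one random goal object, destroying the rest.
; On Tick, the authority copies the time left on the game mode's timeout timer into RemainingTime.
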(event Custom|UpdateSign
  (Networking|SwitchHasAuthority
    (:Authority
      (bind _outactors (Actor|GetAllActorsOfClass "/Game/EyeContact/Blueprints/BP_DirectSign.BP_DirectSign_C"))
      (for _array_element _outactors
        (Default|UpdateSign _array_element)))))

(event EventBeginPlay
  (Networking|SwitchHasAuthority
    (:Authority
      (Utilities|FlowControl|Sequence
        (:then_0
          (CallFunction|SelectEndGoal))
        (:then_1
          (CallFunction|UpdateSign))
        (:then_2
          (CallFunction|SelectGoalObject))))))

(event EventTick
  (params (DeltaSeconds :type Float%20%28single-precision%29))
  (Networking|SwitchHasAuthority
    (:Authority
      (bind _aseye_contact_game_mode (Utilities|Casting|CastToEyeContactGameMode (Game|GetGameMode)))
      (Variables|Default|SetRemainingTime (Utilities|Time|GetTimerRemainingTimebyHandle (Variables|/Game/EyeContact/Blueprints/EyeContactGameMode.EyeContactGameMode_C|GetTimeOutHandle _aseye_contact_game_mode))))))

(fn ConstructionScript)

(fn SelectEndGoal
  ;[1 1 1] Leave only 1 endgoal
  (bind _outactors (Actor|GetAllActorsOfClass "/Game/EyeContact/Blueprints/BP_EndGoal.BP_EndGoal_C"))
  (Variables|Default|SetGoalIndex (Math|Random|RandomIntegerinRange 0 (Utilities|Array|LastIndex _outactors)))
  (for (_array_element _array_index) _outactors
    (if (== _array_index (Variables|Default|GetGoalIndex))
      (Variables|Default|SetActiveEndGoal _array_element)
      (else
        (Game|SpawnActorfromClass "/Game/EyeContact/Blueprints/BP_ExitBlocker.BP_ExitBlocker_C" (Math|Conversions|ToTransform(Vector) (Transformation|GetActorLocation _array_element)) "Undefined" 0 0)
        (Actor|DestroyActor _array_element)))))

(fn SelectGoalObject
  (bind _outactors (Actor|GetAllActorsOfClass "/Game/EyeContact/Blueprints/BP_GoalObject.BP_GoalObject_C"))
  (LocalVariables|SetPickIndex (Math|Random|RandomIntegerinRange 0 (Utilities|Array|LastIndex _outactors)))
  (for (_array_element _array_index) _outactors
    (if (not (== _array_index (LocalVariables|GetPickIndex)))
      (Actor|DestroyActor _array_element))))