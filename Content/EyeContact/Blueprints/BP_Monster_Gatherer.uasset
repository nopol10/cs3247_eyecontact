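; BP_Monster_Gatherer is the gatherer monster, with an echolocation skill that targets human players.
; Echolocation calls EchoHit on every BP_HumanPlayer with a highlight duration, then starts SkillTimer.
; Tick counts the timer up to SkillDuration and resets it to zero, which marks the skill as ready.
; The cooldown-gated skill trigger has no connected event, so echolocation never fires from this graph.
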(event EventBeginPlay
  (|CallParentFunction)
  (Variables|Default|SetSkillTimer 0.0)
  (Development|PrintString "Monster gatherer"))

(event Collision|EventActorBeginOverlap
  (params (OtherActor :type Actor%20Object%20Reference)))

(event EventTick
  (params (DeltaSeconds :type Float%20%28single-precision%29))
  (|CallParentFunction DeltaSeconds)
  (CallFunction|UpdateSkillTimer DeltaSeconds))

(fn ConstructionScript
  (|CallParentFunction))

(fn UpdateSkillTimer
  (params (DeltaTime :type Float%20%28single-precision%29))
  (if (> (Variables|Default|GetSkillTimer) 0.0)
    (if (>= (Variables|Default|GetSkillTimer) (Variables|Default|GetSkillDuration))
      (Variables|Default|SetSkillTimer 0.0)
      (Development|PrintString "SkillReady")
      (else
        (Variables|Default|SetSkillTimer (+ (Variables|Default|GetSkillTimer) DeltaTime)))))
  (return))

(fn Echolocation
  (bind _outactors (Actor|GetAllActorsOfClass "/Game/EyeContact/Blueprints/BP_HumanPlayer.BP_HumanPlayer_C"))
  (for _array_element _outactors
    (bind _asbp_human_player (Utilities|Casting|CastToBP_HumanPlayer _array_element))
    (Default|EchoHit _asbp_human_player (Variables|Default|GetEchoHighlightDuration)))
  (Development|PrintString "Start echolocation!")
  (Variables|Default|SetSkillTimer 0.01)
  (return))