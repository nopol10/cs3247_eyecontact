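; BP_InstanceTester is a debug Blueprint that checks team assignments stored in BP_EyeContactGameInstance.
; On BeginPlay, only on authority, it looks up each BP_EyeContactController's PlayerId in the human and monster ID arrays.
; It prints whether each player is human, monster or unknown.
; Leftover loops and player-state lookups are disconnected.
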(event EventBeginPlay
  (Networking|SwitchHasAuthority
    (:Authority
      (bind _outactors (Actor|GetAllActorsOfClass "/Game/EyeContact/Blueprints/BP_EyeContactController.BP_EyeContactController_C"))
      (bind _asbp_eye_contact_game_instance (Utilities|Casting|CastToBP_EyeContactGameInstance (Game|GetGameInstance)))
      (for _array_element _outactors
        (if (< (Utilities|Array|FindItem (Variables|/Game/EyeContact/Blueprints/BP_EyeContactGameInstance.BP_EyeContactGameInstance_C|GetHumanPlayerIds _asbp_eye_contact_game_instance) (Variables|/Script/Engine.PlayerState|GetPlayerId (Variables|/Script/Engine.Controller|GetPlayerState _array_element))) 0)
          (if (< (Utilities|Array|FindItem (Variables|/Game/EyeContact/Blueprints/BP_EyeContactGameInstance.BP_EyeContactGameInstance_C|GetMonsterPlayerIds _asbp_eye_contact_game_instance) (Variables|/Script/Engine.PlayerState|GetPlayerId (Variables|/Script/Engine.Controller|GetPlayerState _array_element))) 0)
            (Development|PrintString "No idea what this is")
            (else
              (Development|PrintString (Utilities|String|Append (Utilities|String|ToString(Integer) (Variables|/Script/Engine.PlayerState|GetPlayerId (Variables|/Script/Engine.Controller|GetPlayerState _array_element))) " is a monster"))))
          (else
            (Development|PrintString (Utilities|String|Append (Utilities|String|ToString(Integer) (Variables|/Script/Engine.PlayerState|GetPlayerId (Variables|/Script/Engine.Controller|GetPlayerState _array_element))) " is human"))))))))

(fn ConstructionScript)