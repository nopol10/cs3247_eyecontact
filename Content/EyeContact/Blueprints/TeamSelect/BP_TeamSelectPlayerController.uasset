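; Player controller for the team selection screen, turning menu inputs into team indicator moves and mode changes.
; On InitializePlayer it asks the EyeContactTeamSelectMode game mode to spawn its select pawn.
; Left and right inputs forward the controller to TeamSelectGameState to move its indicator.
; Game mode switching and the Interaction confirm press run only with authority, calling UpdateUIMode and EnterPressed on that game state.
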(event Custom|MoveRightPC
  ;[1 1 1] Selector Movement
  (bind _asteam_select_game_state (Utilities|Casting|CastToTeamSelectGameState (Game|GetGameState)))
  (Default|MoveIndicatorRight _asteam_select_game_state self))

(event Custom|InitializePlayer
  (bind _aseye_contact_team_select_mode (Utilities|Casting|CastToEyeContactTeamSelectMode (Game|GetGameMode)))
  (Default|SpawnSelectPawn _aseye_contact_team_select_mode self))

(event Custom|MoveLeftPC
  ;[1 1 1] Selector Movement
  (bind _asteam_select_game_state (Utilities|Casting|CastToTeamSelectGameState (Game|GetGameState)))
  (Default|MoveIndicatorLeft _asteam_select_game_state self))

(event Custom|SwitchGameMode
  ;[1 1 1] Selector Movement
  (bind _asteam_select_game_state (Utilities|Casting|CastToTeamSelectGameState (Game|GetGameState)))
  (Default|UpdateUIMode _asteam_select_game_state))

(event EventBeginPlay)

(event EventTick
  (params (DeltaSeconds :type Float%20%28single-precision%29)))

(event Input|ActionEvents|InputActionMenuRight
  (params (Key :type Key%20Structure :default "AnyKey"))
  ;[1 1 1] Selector Movement
  (:Pressed
    (CallFunction|MoveRightPC)))

(event Input|ActionEvents|InputActionMenuSwitchGameMode
  (params (Key :type Key%20Structure :default "AnyKey"))
  ;[1 1 1] Selector Movement
  (:Pressed
    (Networking|SwitchHasAuthority
      (:Authority
        (CallFunction|SwitchGameMode)))))

(event Input|ActionEvents|InputActionInteraction
  (params (Key :type Key%20Structure :default "AnyKey"))
  ;[1 1 1] Selector Movement
  (:Pressed
    (Networking|SwitchHasAuthority
      (:Authority
        (bind _asteam_select_game_state (Utilities|Casting|CastToTeamSelectGameState (Game|GetGameState)))
        (Default|EnterPressed _asteam_select_game_state)))))

(event Input|ActionEvents|InputActionMenuLeft
  (params (Key :type Key%20Structure :default "AnyKey"))
  ;[1 1 1] Selector Movement
  (:Pressed
    (CallFunction|MoveLeftPC)))

(fn ConstructionScript)