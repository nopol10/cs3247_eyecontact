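; Pawn for the team selection screen that the player shifts sideways with menu input.
; On BeginPlay it prints the session's server name and player count from the EyeContact game instance, then switches the first player controller to game-only input.
; MenuLeft teleports it a fixed step along negative Y with SetActorLocation; no rightward input is handled, and alternative movement nodes are left disconnected.
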(event Custom|CustomEvent_0)

(event EventBeginPlay
  (bind _asbp_eye_contact_game_instance (Utilities|Casting|CastToBP_EyeContactGameInstance (Game|GetGameInstance)))
  (Development|PrintString (Utilities|String|Append (Class|FindSessionsCallbackProxy|GetServerName (Variables|/Game/EyeContact/Blueprints/BP_EyeContactGameInstance.BP_EyeContactGameInstance_C|GetSessionInfo _asbp_eye_contact_game_instance)) " ---------- " (Utilities|String|ToString(Integer) (Class|FindSessionsCallbackProxy|GetCurrentPlayers (Variables|/Game/EyeContact/Blueprints/BP_EyeContactGameInstance.BP_EyeContactGameInstance_C|GetSessionInfo _asbp_eye_contact_game_instance)))))
  (Input|SetInputModeGameOnly (Game|GetPlayerController 0)))

(event EventActorBeginOverlap
  (params (OtherActor :type Actor%20Object%20Reference)))

(event EventTick
  (params (DeltaSeconds :type Float%20%28single-precision%29)))

(event Input|ActionEvents|InputActionMenuLeft
  (params (Key :type Key%20Structure :default "AnyKey"))
  (:Pressed
    (Transformation|SetActorLocation (- (Transformation|GetActorLocation) "0,300.000000, 0") false false)))

(fn ConstructionScript)