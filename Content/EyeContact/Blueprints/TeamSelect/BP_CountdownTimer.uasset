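; BP_CountdownTimer is a team-select actor that shows a countdown as a whole number of seconds on a text element.
; While enabled, the authority reduces CountdownTime each Tick, clamps it at zero, refreshes the text, then fires OnTimerEnd once and disables itself.
; CountdownTime replicates through a RepNotify, so clients update their displayed text from the server's value.
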(event EventBeginPlay)

(event EventActorBeginOverlap
  (params (OtherActor :type Actor%20Object%20Reference)))

(event EventTick
  (params (DeltaSeconds :type Float%20%28single-precision%29))
  (if (and (Variables|Default|GetCountdownEnabled) (Ability|HasAuthority))
    (bind _output_get (Variables|Default|SetCountdownTime (Math|Float|Clamp(Float) (- (Variables|Default|GetCountdownTime) DeltaSeconds) 0.0 (Variables|Default|GetCountdownTime))))
    (CallFunction|UpdateTimer)
    (if (<= _output_get 0.0)
      (Default|CallOnTimerEnd)
      (Variables|Default|SetCountdownEnabled false))))

(fn ConstructionScript)

(fn UpdateTimer
  (Rendering|Components|TextRender|SetText (Variables|Default|GetTimerText) (Utilities|Text|ToText(Integer) (Math|Float|Round (Variables|Default|GetCountdownTime)))))

(fn OnRepCountdownTime
  (CallFunction|UpdateTimer))