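; Class selection pedestal for team select that previews the human or monster character meshes available for its Type.
; CycleClass steps SelectedIndex left or right with wraparound through HumanMeshes or MonsterMeshes and stores the chosen entry in DisplayMeshVariable.
; That variable's RepNotify applies the entry's skeletal mesh and animation Blueprint to DisplayMesh, so the displayed character follows replication.
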(event Custom|CycleClass
  (params (CycleLeft :type Boolean))
  (if (Utilities|Enum|Equal(Enum) (Variables|Default|GetType) "NewEnumerator0")
    (Variables|Default|SetMaxMeshLength (Utilities|Array|Length (Variables|Default|GetHumanMeshes)))
    (else
      (Variables|Default|SetMaxMeshLength (Utilities|Array|Length (Variables|Default|GetMonsterMeshes)))))
  (if CycleLeft
    (if (< (- (Variables|Default|GetSelectedIndex) 1) 0)
      (Variables|Default|SetSelectedIndex (- (Variables|Default|GetMaxMeshLength) 1))
      (else
        (Variables|Default|SetSelectedIndex (Math|Integer|%(Integer) (- (Variables|Default|GetSelectedIndex) 1) (Variables|Default|GetMaxMeshLength)))))
    (else
      (Variables|Default|SetSelectedIndex (Math|Integer|%(Integer) (+ (Variables|Default|GetSelectedIndex) 1) (Variables|Default|GetMaxMeshLength)))))
  (if (Utilities|Enum|Equal(Enum) (Variables|Default|GetType) "NewEnumerator0")
    (Development|PrintString (Utilities|String|ToString(Integer) (Variables|Default|GetSelectedIndex)))
    ;[1 1 1] Set Human Mesh
    (Variables|Default|SetDisplayMeshVariable (Utilities|Array|Get(acopy) (Variables|Default|GetHumanMeshes) (Variables|Default|GetSelectedIndex)))
    (else
      ;[1 1 1] Set Human Mesh
      (Variables|Default|SetDisplayMeshVariable (Utilities|Array|Get(acopy) (Variables|Default|GetMonsterMeshes) (Variables|Default|GetSelectedIndex))))))

(event EventBeginPlay)

(event Collision|EventActorBeginOverlap
  (params (OtherActor :type Actor%20Object%20Reference)))

(event EventTick
  (params (DeltaSeconds :type Float%20%28single-precision%29)))

(fn ConstructionScript)

(fn OnRepDisplayMeshVariable
  (bind _displaymesh (Variables|Default|GetDisplayMesh))
  (bind _displaymeshvariable (Variables|Default|GetDisplayMeshVariable))
  ;[1 1 1] Set Human Mesh
  (Class|SkinnedMeshComponent|SetSkeletalMesh _displaymesh (.skeletalmesh _displaymeshvariable) true)
  (Components|SkeletalMesh|SetAnimInstanceClass _displaymesh (.animationblueprint _displaymeshvariable)))