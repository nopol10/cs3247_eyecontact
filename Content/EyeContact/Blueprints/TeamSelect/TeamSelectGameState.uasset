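; Game state for the team select lobby, where players pick Human or Monster before a match.
; Left/right moves shift each player's indicator and update size-capped team arrays, refreshing the count text in the 3D lobby widget, with OnRep functions updating client UI.
; When the server-bound countdown ends, it places unassigned players on Humans, overflowing to Monsters, saves both teams' player IDs to the game instance and server-travels to EC_TestLevel.
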(event Custom|CountdownComplete
  (CallFunction|OnCountdownComplete))

(event Custom|MoveIndicatorLeft
  (params (PlayerController :type Player%20Controller%20Object%20Reference))
  (bind _playercontrollers (Variables|Default|GetPlayerControllers))
  (bind _indicators (Variables|Default|GetIndicators))
  (bind _returnvalue (Utilities|Array|FindItem _playercontrollers PlayerController))
  (bind _item (Utilities|Array|Get(acopy) _indicators _returnvalue))
  (bind _selectiontype (CallFunction|GetCurrentSelection PlayerController))
  (switch Utilities|FlowControl|Switch|SwitchonEPlayerType _selectiontype
    (:NewEnumerator1
      ;[1 1 1] Remove from Monster Team
      (Transformation|AddActorWorldOffset _item "0,-300.000000, 0")
      (Utilities|Array|RemoveItem (Variables|Default|GetMonsterPlayers) (Variables|/Script/Engine.Controller|GetPlayerState PlayerController))
      (CallFunction|UpdateTeamSelectUIServer :!label _label))
    (:NewEnumerator2
      ;[1 1 1] Set player to Humans
      (if (< (Utilities|Array|Length (Variables|Default|GetHumanPlayers)) (Variables|Default|GetMaxHumanPlayerCount))
        (Transformation|AddActorWorldOffset _item "0,-300.000000, 0")
        (Utilities|Array|Add (Variables|Default|GetHumanPlayers) (Variables|/Script/Engine.Controller|GetPlayerState PlayerController))
        (goto _label)))))

(event Custom|MoveIndicatorRight
  (params (PlayerController :type Player%20Controller%20Object%20Reference))
  (bind _playercontrollers (Variables|Default|GetPlayerControllers))
  (bind _indicators (Variables|Default|GetIndicators))
  (bind _returnvalue (Utilities|Array|FindItem _playercontrollers PlayerController))
  (bind _item (Utilities|Array|Get(acopy) _indicators _returnvalue))
  (bind _selectiontype (CallFunction|GetCurrentSelection PlayerController))
  (switch Utilities|FlowControl|Switch|SwitchonEPlayerType _selectiontype
    (:NewEnumerator0
      ;[1 1 1] Remove from Human Team
      (Transformation|AddActorWorldOffset _item "0,300.000000, 0")
      (Utilities|Array|RemoveItem (Variables|Default|GetHumanPlayers) (Variables|/Script/Engine.Controller|GetPlayerState PlayerController))
      (CallFunction|UpdateTeamSelectUIServer :!label _label))
    (:NewEnumerator2
      ;[1 1 1] Set player to Monster
      (if (< (Utilities|Array|Length (Variables|Default|GetMonsterPlayers)) (Variables|Default|GetMaxMonsterPlayerCount))
        (Transformation|AddActorWorldOffset _item "0,300.000000, 0")
        (Utilities|Array|Add (Variables|Default|GetMonsterPlayers) (Variables|/Script/Engine.Controller|GetPlayerState PlayerController))
        (goto _label)))))

(event EventBeginPlay
  ;[1 1 1] Get Widget stuff
  (bind _outactors (Actor|GetAllActorsOfClass "/Game/EyeContact/Blueprints/TeamSelect/BP_SelectTeamWidget3D.BP_SelectTeamWidget3D_C"))
  (bind _asw_waiting_for_player_dialog (Utilities|Casting|CastToW_WaitingForPlayerDialog (UserInterface|GetUserWidgetObject (Variables|/Game/EyeContact/Blueprints/TeamSelect/BP_SelectTeamWidget3D.BP_SelectTeamWidget3D_C|GetLobbyMenu (Utilities|Array|Get(acopy) _outactors)))))
  (Variables|Default|SetTeamSelectUI _asw_waiting_for_player_dialog)
  (Networking|SwitchHasAuthority
    (:Authority
      (bind _outactors_2 (Actor|GetAllActorsOfClass "/Game/EyeContact/Blueprints/TeamSelect/BP_CountdownTimer.BP_CountdownTimer_C"))
      (EventDispatchers|BindEventtoOnTimerEnd (Utilities|Array|Get(acopy) _outactors_2) (delegate Custom|CountdownComplete)))))

(fn ConstructionScript)

(fn GetCurrentSelection
  (params (PlayerController :type Player%20Controller%20Object%20Reference))
  (bind _playerstate (Variables|/Script/Engine.Controller|GetPlayerState PlayerController))
  (if (< (Utilities|Array|FindItem (Variables|Default|GetHumanPlayers) _playerstate) 0)
    (if (< (Utilities|Array|FindItem (Variables|Default|GetMonsterPlayers) _playerstate) 0)
      (return "NewEnumerator2")
      (else
        (return "NewEnumerator1")))
    (else
      (return "NewEnumerator0"))))

(fn UpdateTeamSelectUIServer
  (bind _humanplayers (Variables|Default|GetHumanPlayers))
  (bind _maxhumanplayercount (Variables|Default|GetMaxHumanPlayerCount))
  (bind _monsterplayers (Variables|Default|GetMonsterPlayers))
  (bind _maxmonsterplayercount (Variables|Default|GetMaxMonsterPlayerCount))
  (bind _returnvalue (Utilities|Array|Length _monsterplayers))
  (bind _returnvalue_2 (Utilities|Array|Length _humanplayers))
  (bind _returnvalue_3 (Utilities|String|ToString(Integer) _maxmonsterplayercount))
  (bind _returnvalue_4 (Utilities|String|ToString(Integer) _maxhumanplayercount))
  (bind _returnvalue_5 (Utilities|String|ToString(Integer) _returnvalue))
  (bind _returnvalue_6 (Utilities|String|ToString(Integer) _returnvalue_2))
  (bind _returnvalue_7 (Utilities|String|Append _returnvalue_5 "/" _returnvalue_3))
  (bind _returnvalue_8 (Utilities|String|Append _returnvalue_6 "/" _returnvalue_4))
  (Variables|Default|SetHumanCountText _returnvalue_8)
  (Rendering|Components|TextRender|SetText (Variables|/Game/EyeContact/Interface/W_WaitingForPlayerDialog.W_WaitingForPlayerDialog_C|GetHumanCountText (Variables|Default|GetTeamSelectUI)) (Utilities|Text|ToText(String) _returnvalue_8))
  (Variables|Default|SetMonsterCountText _returnvalue_7)
  (Rendering|Components|TextRender|SetText (Variables|/Game/EyeContact/Interface/W_WaitingForPlayerDialog.W_WaitingForPlayerDialog_C|GetMonsterCountText (Variables|Default|GetTeamSelectUI)) (Utilities|Text|ToText(String) _returnvalue_7)))

(fn OnRepHumanCountTextBox
  (CallFunction|UpdateClientUI))

(fn OnRepMonsterCountTextBox
  (CallFunction|UpdateClientUI))

(fn UpdateClientUI
  (Rendering|Components|TextRender|SetText (Variables|/Game/EyeContact/Interface/W_WaitingForPlayerDialog.W_WaitingForPlayerDialog_C|GetHumanCountText (Variables|Default|GetTeamSelectUI)) (Utilities|Text|ToText(String) (Variables|Default|GetHumanCountText)))
  (Rendering|Components|TextRender|SetText (Variables|/Game/EyeContact/Interface/W_WaitingForPlayerDialog.W_WaitingForPlayerDialog_C|GetMonsterCountText (Variables|Default|GetTeamSelectUI)) (Utilities|Text|ToText(String) (Variables|Default|GetMonsterCountText))))

(fn OnCountdownComplete
  (bind _humanplayers (Variables|Default|GetHumanPlayers))
  (Utilities|FlowControl|Sequence
    (:then_0
      ;[1 1 1] Check for unassigned players
      (for _array_element (Variables|Default|GetPlayerControllers)
        (bind _selectiontype (CallFunction|GetCurrentSelection _array_element))
        (switch Utilities|FlowControl|Switch|SwitchonEPlayerType _selectiontype
          (:NewEnumerator2
            (if (< (Utilities|Array|Length _humanplayers) (Variables|Default|GetMaxHumanPlayerCount))
              ;[1 1 1] Human team still has space
              (Utilities|Array|Add _humanplayers (Variables|/Script/Engine.Controller|GetPlayerState _array_element))
              (else
                ;[1 1 1] Force into monster team for now
                (Utilities|Array|Add (Variables|Default|GetMonsterPlayers) 0)))))))
    (:then_1
      (bind _asbp_eye_contact_game_instance (Utilities|Casting|CastToBP_EyeContactGameInstance (Game|GetGameInstance)))
      (Utilities|Array|Clear (Variables|/Game/EyeContact/Blueprints/BP_EyeContactGameInstance.BP_EyeContactGameInstance_C|GetHumanPlayerIds _asbp_eye_contact_game_instance))
      (Utilities|Array|Clear (Variables|/Game/EyeContact/Blueprints/BP_EyeContactGameInstance.BP_EyeContactGameInstance_C|GetMonsterPlayerIds _asbp_eye_contact_game_instance)))
    (:then_2
      (for _array_element_2 (Variables|Default|GetHumanPlayers)
        (Utilities|Array|Add (Variables|/Game/EyeContact/Blueprints/BP_EyeContactGameInstance.BP_EyeContactGameInstance_C|GetHumanPlayerIds _asbp_eye_contact_game_instance) (Variables|/Script/Engine.PlayerState|GetPlayerId _array_element_2))))
    (:then_3
      (for _array_element_3 (Variables|Default|GetMonsterPlayers)
        (Utilities|Array|Add (Variables|/Game/EyeContact/Blueprints/BP_EyeContactGameInstance.BP_EyeContactGameInstance_C|GetMonsterPlayerIds _asbp_eye_contact_game_instance) (Variables|/Script/Engine.PlayerState|GetPlayerId _array_element_3))))
    (:then_4
      (Development|ExecuteConsoleCommand "servertravel EC_TestLevel"))))