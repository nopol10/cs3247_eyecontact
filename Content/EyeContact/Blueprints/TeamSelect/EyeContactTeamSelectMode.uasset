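; Game mode for team selection that keeps a selecting indicator for each player controller in the TeamSelectGameState.
; SpawnSelectPawn registers the controller and spawns a name-labelled indicator at the first BP_SpawnLocation, stacked downward by player index.
; OnLogout, on authority, destroys that indicator and removes the controller, but looks up the indicator's array index after that removal.
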(event Custom|SpawnSelectPawn
  (params (New%20Player :type Player%20Controller%20Object%20Reference))
  (bind _asteam_select_game_state (Utilities|Casting|CastToTeamSelectGameState (Game|GetGameState)))
  (Variables|Default|SetTeamSelectState _asteam_select_game_state)
  (bind _outactors (Actor|GetAllActorsOfClass "/Game/EyeContact/Blueprints/TeamSelect/BP_SpawnLocation.BP_SpawnLocation_C"))
  (Variables|/Game/EyeContact/Blueprints/TeamSelect/TeamSelectGameState.TeamSelectGameState_C|SetSpawnLocation _asteam_select_game_state (Utilities|Array|Get(acopy) _outactors))
  (bind _returnvalue (Utilities|Array|Add (Variables|/Game/EyeContact/Blueprints/TeamSelect/TeamSelectGameState.TeamSelectGameState_C|GetPlayerControllers (Variables|Default|GetTeamSelectState)) New%20Player))
  (bind _returnvalue_2 (Game|SpawnActorfromClass "/Game/EyeContact/Blueprints/TeamSelect/BP_SelectingIndicator.BP_SelectingIndicator_C" (Math|Conversions|ToTransform(Vector) (+ (Transformation|GetActorLocation (Variables|/Game/EyeContact/Blueprints/TeamSelect/TeamSelectGameState.TeamSelectGameState_C|GetSpawnLocation (Variables|Default|GetTeamSelectState))) (* "0, 0,-80.000000" _returnvalue))) "Undefined" 0 0))
  (Utilities|Array|Add (Variables|/Game/EyeContact/Blueprints/TeamSelect/TeamSelectGameState.TeamSelectGameState_C|GetIndicators (Variables|Default|GetTeamSelectState)) _returnvalue_2)
  (Variables|/Game/EyeContact/Blueprints/TeamSelect/BP_SelectingIndicator.BP_SelectingIndicator_C|SetPlayerNameString _returnvalue_2 (Variables|/Script/Engine.PlayerState|GetPlayerName (Variables|/Script/Engine.Controller|GetPlayerState New%20Player))))

(event EventBeginPlay
  (bind _asteam_select_game_state (Utilities|Casting|CastToTeamSelectGameState (Game|GetGameState)))
  (bind _output_get (Variables|Default|SetTeamSelectState _asteam_select_game_state))
  (bind _outactors (Actor|GetAllActorsOfClass "/Game/EyeContact/Blueprints/TeamSelect/BP_SpawnLocation.BP_SpawnLocation_C"))
  (Variables|/Game/EyeContact/Blueprints/TeamSelect/TeamSelectGameState.TeamSelectGameState_C|SetSpawnLocation _output_get (Utilities|Array|Get(acopy) _outactors)))

(event EventTick
  (params (DeltaSeconds :type Float%20%28single-precision%29)))

(event EventPostLogin
  (params (NewPlayer :type Player%20Controller%20Object%20Reference)))

(event EventOnLogout
  (params (ExitingController :type Controller%20Object%20Reference))
  (bind _teamselectstate (Variables|Default|GetTeamSelectState))
  (bind _playercontrollers (Variables|/Game/EyeContact/Blueprints/TeamSelect/TeamSelectGameState.TeamSelectGameState_C|GetPlayerControllers _teamselectstate))
  (bind _indicators (Variables|/Game/EyeContact/Blueprints/TeamSelect/TeamSelectGameState.TeamSelectGameState_C|GetIndicators _teamselectstate))
  (Networking|SwitchHasAuthority
    (:Authority
      (bind _returnvalue (Utilities|Casting|CastToPlayerController ExitingController))
      (Actor|DestroyActor (Utilities|Array|Get(acopy) _indicators (Utilities|Array|FindItem _playercontrollers _returnvalue)))
      (Utilities|Array|RemoveItem _playercontrollers _returnvalue)
      (Utilities|Array|RemoveIndex _indicators (Utilities|Array|FindItem _playercontrollers _returnvalue)))))

(fn ConstructionScript)