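; BP_Switch is an interactable light switch that turns a linked light object on and off.
; Interact toggles LightOn on authority, and its RepNotify sets light visibility and moves and recolors the button, which glows red when off.
; BeginPlay sets LightOn if the light starts visible.
; Box overlap by human or monster players toggles custom depth rendering on the switch meshes for highlighting.
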(event OnComponentBeginOverlap(Box)
  (params (OverlappedComponent :type Primitive%20Component%20Object%20Reference) (OtherActor :type Actor%20Object%20Reference) (OtherComp :type Primitive%20Component%20Object%20Reference) (OtherBodyIndex :type Integer) (bFromSweep :type Boolean) (SweepResult :type Hit%20Result%20Structure%20%28by%20ref%29))
  (Utilities|Casting|CastToBP_HumanPlayer OtherActor
    (:then
      _)
    (:CastFailed
      (Utilities|Casting|CastToBP_MonsterPlayer OtherActor)))
  (Rendering|SetRenderCustomDepth (Variables|Default|GetSwitchBody) true)
  (Rendering|SetRenderCustomDepth (Variables|Default|GetSwitchButton) true))

(event OnComponentEndOverlap(Box)
  (params (OverlappedComponent :type Primitive%20Component%20Object%20Reference) (OtherActor :type Actor%20Object%20Reference) (OtherComp :type Primitive%20Component%20Object%20Reference) (OtherBodyIndex :type Integer))
  (Utilities|Casting|CastToBP_HumanPlayer OtherActor
    (:then
      _)
    (:CastFailed
      (Utilities|Casting|CastToBP_MonsterPlayer OtherActor)))
  (Rendering|SetRenderCustomDepth (Variables|Default|GetSwitchBody) false)
  (Rendering|SetRenderCustomDepth (Variables|Default|GetSwitchButton) false))

(event EventInteract
  (params (Interactor :type Actor%20Object%20Reference))
  (Networking|SwitchHasAuthority
    (:Authority
      (if (Variables|Default|GetLightOn)
        (Variables|Default|SetLightOn false)
        (else
          (Variables|Default|SetLightOn true))))))

(event EventBeginPlay
  (if (Rendering|IsVisible (Variables|/Script/Engine.Light|GetLightComponent (Variables|Default|GetLightObject)))
    (Variables|Default|SetLightOn true)))

(event EventActorBeginOverlap
  (params (OtherActor :type Actor%20Object%20Reference)))

(event EventTick
  (params (DeltaSeconds :type Float%20%28single-precision%29)))

(fn ConstructionScript)

(fn OnRepLighton
  (bind _lightobject (Variables|Default|GetLightObject))
  (bind _lightcomponent (Variables|/Script/Engine.Light|GetLightComponent _lightobject))
  (if (Variables|Default|GetLightOn)
    (CallFunction|PressSwitch)
    (Rendering|SetVisibility _lightcomponent true false)
    (else
      (CallFunction|DepressSwitch)
      (Rendering|SetVisibility _lightcomponent false false))))

(fn PressSwitch
  (bind _switchbutton (Variables|Default|GetSwitchButton))
  (Transformation|SetRelativeLocation _switchbutton (Variables|Default|GetOnLocation) false false)
  (Rendering|Material|SetMaterial _switchbutton 0 "/Game/LayoutAssets/Materials/M_Color_Black.M_Color_Black"))

(fn DepressSwitch
  (Transformation|SetRelativeLocation (Variables|Default|GetSwitchButton) (Variables|Default|GetOffLocation) false false)
  (Rendering|Material|SetMaterial (Variables|Default|GetSwitchButton) 0 "/Game/LayoutAssets/Materials/M_Emissive_Red.M_Emissive_Red"))