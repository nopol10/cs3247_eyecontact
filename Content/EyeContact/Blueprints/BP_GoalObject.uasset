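; BP_GoalObject is the objective pickup that human players collect in EyeContact.
; Box overlap by player pawn 0, if able to move on entry, toggles the cylinder's custom-depth highlight and timeline-scales prompt text that turns toward that player.
; On Interact, the server flags the game mode and interacting player as holding the goal, spawns an emitter, makes all monsters roar, then destroys the object.
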(event OnComponentBeginOverlap(Box)
  (params (OtherActor :type Actor%20Object%20Reference) (OtherComp :type Primitive%20Component%20Object%20Reference) (OtherBodyIndex :type Integer) (bFromSweep :type Boolean) (SweepResult :type Hit%20Result%20Structure%20%28by%20ref%29))
  (bind _asbp_human_player (Utilities|Casting|CastToBP_HumanPlayer OtherActor))
  (bind _canmove (Default|CanMove _asbp_human_player))
  (if (and (== _asbp_human_player (Game|Player|GetPlayerPawn 0)) _canmove)
    (Rendering|SetRenderCustomDepth (Variables|Default|GetCylinder) true)
    (CallFunction|ResetTimeline (Variables|Default|GetScaleUp))
    (CallFunction|ResetTimeline (Variables|Default|GetScaleDown))
    (Utilities|FlowControl|Sequence
      (:then_0
        (bind _scale (Timeline|ScaleUp Play)
          (:Update
            (Transformation|SetWorldScale3D (Variables|Default|GetInteractText) (Math|Vector|MakeVector _scale _scale _scale)))))
      (:then_1
        (Variables|Default|SetIsPlayerInZone true)))))

(event OnComponentEndOverlap(Box)
  (params (OtherActor :type Actor%20Object%20Reference) (OtherComp :type Primitive%20Component%20Object%20Reference) (OtherBodyIndex :type Integer))
  (bind _asbp_human_player (Utilities|Casting|CastToBP_HumanPlayer OtherActor))
  (if (== _asbp_human_player (Game|Player|GetPlayerPawn 0))
    (Rendering|SetRenderCustomDepth (Variables|Default|GetCylinder) false)
    (CallFunction|ResetTimeline (Variables|Default|GetScaleUp))
    (CallFunction|ResetTimeline (Variables|Default|GetScaleDown))
    (Utilities|FlowControl|Sequence
      (:then_0
        (bind _scale (Timeline|ScaleDown Play)
          (:Update
            (Transformation|SetWorldScale3D (Variables|Default|GetInteractText) (Math|Vector|MakeVector _scale _scale _scale)))))
      (:then_1
        (Variables|Default|SetIsPlayerInZone false)))))

(event EventInteract
  (params (Interactor :type Actor%20Object%20Reference))
  (Development|PrintString (Utilities|GetDisplayName Interactor))
  (Networking|SwitchHasAuthority
    (:Authority
      (bind _aseye_contact_game_mode (Utilities|Casting|CastToEyeContactGameMode (Game|GetGameMode)))
      (Utilities|FlowControl|Sequence
        (:then_0
          (Variables|/Game/EyeContact/Blueprints/EyeContactGameMode.EyeContactGameMode_C|SetHumansHaveGoal _aseye_contact_game_mode true)
          (Default|SpawnEmitter _aseye_contact_game_mode "/Game/EyeContact/Particles/AttractiveParticle.AttractiveParticle" (Transformation|GetActorLocation)))
        (:then_1
          (Default|AllMonstersRoar _aseye_contact_game_mode))
        (:then_2
          (bind _asbp_human_player (Utilities|Casting|CastToBP_HumanPlayer Interactor))
          (Variables|/Game/EyeContact/Blueprints/BP_HumanPlayer.BP_HumanPlayer_C|SetHasGoalObject _asbp_human_player true))
        (:then_3
          (Actor|DestroyActor))))))

(event EventBeginPlay
  (Transformation|SetWorldScale3D (Variables|Default|GetInteractText) "0, 0, 0"))

(event EventActorBeginOverlap
  (params (OtherActor :type Actor%20Object%20Reference)))

(event EventTick
  (params (DeltaSeconds :type Float%20%28single-precision%29))
  (CallFunction|FaceObject (Variables|Default|GetInteractText) (Game|Player|GetPlayerPawn 0)))

(fn ConstructionScript)