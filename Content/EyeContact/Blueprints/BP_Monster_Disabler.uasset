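; BP_Monster_Disabler is a monster character Blueprint, apparently built around roar and blind disabling skills.
; Its RoarSphere overlap events maintain PossibleRoarStun, the human players within roar stun range, with debug prints on changes.
; The Roar and Blind calls sit in disconnected cooldown-check branches that never run, so this graph only tracks stun candidates.
; BeginPlay, Tick and construction defer to the parent, with BeginPlay also printing a "Monster gatherer" debug label.
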(event OnComponentEndOverlap(RoarSphere)
  (params (OverlappedComponent :type Primitive%20Component%20Object%20Reference) (OtherActor :type Actor%20Object%20Reference) (OtherComp :type Primitive%20Component%20Object%20Reference) (OtherBodyIndex :type Integer))
  ;[1 1 1] Roar stun area of effect
  (bind _asbp_human_player (Utilities|Casting|CastToBP_HumanPlayer OtherActor))
  (Utilities|Array|RemoveItem (Variables|Default|GetPossibleRoarStun) _asbp_human_player)
  (Development|PrintString "Exit"))

(event OnComponentBeginOverlap(RoarSphere)
  (params (OverlappedComponent :type Primitive%20Component%20Object%20Reference) (OtherActor :type Actor%20Object%20Reference) (OtherComp :type Primitive%20Component%20Object%20Reference) (OtherBodyIndex :type Integer) (bFromSweep :type Boolean) (SweepResult :type Hit%20Result%20Structure%20%28by%20ref%29))
  ;[1 1 1] Roar stun area of effect
  (bind _asbp_human_player (Utilities|Casting|CastToBP_HumanPlayer OtherActor))
  (bind _returnvalue (Utilities|Array|Add (Variables|Default|GetPossibleRoarStun) _asbp_human_player))
  (Development|PrintString (Utilities|String|ToString(Integer) _returnvalue)))

(event EventBeginPlay
  (|CallParentFunction)
  (Development|PrintString "Monster gatherer"))

(event EventTick
  (params (DeltaSeconds :type Float%20%28single-precision%29))
  (|CallParentFunction DeltaSeconds))

(fn ConstructionScript
  (|CallParentFunction))