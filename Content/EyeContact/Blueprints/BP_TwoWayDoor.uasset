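; BP_TwoWayDoor is a replicated interactable door that can swing open in either of two directions.
; On the server, Interact closes an open door, or opens it front or back according to which side volume overlaps the interactor.
; RepNotifies on the two open-state booleans call OpenFront and OpenBack, which play or reverse separate timelines that lerp the door body's relative rotation.
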(event EventBeginPlay)

(event EventActorBeginOverlap
  (params (OtherActor :type Actor%20Object%20Reference)))

(event EventTick
  (params (DeltaSeconds :type Float%20%28single-precision%29)))

(fn ConstructionScript)

(fn OnRepDoorOpenFront
  (CallFunction|OpenFront))

(fn OnRepDoorOpenBack
  (CallFunction|OpenBack))

(event Custom|Open%20Front
  (if (Variables|Default|GetDoorOpenFront)
    (bind _doormovement (Timeline|Timeline_0 ReverseFromEnd)
      (:Update
        (Transformation|SetRelativeRotation (Variables|Default|GetDoorBody) (Math|Rotator|Lerp(Rotator) (Variables|Default|GetFrontRotation) "0, 0, 0" _doormovement) false false)))
    (else
      (Timeline|Timeline_0 PlayFromStart))))

(event EventInteract
  (params (Interactor :type Actor%20Object%20Reference))
  (Networking|SwitchHasAuthority
    (:Authority
      (if (or (Variables|Default|GetDoorOpenBack) (Variables|Default|GetDoorOpenFront))
        (if (Variables|Default|GetDoorOpenFront)
          (Variables|Default|SetDoorOpenFront false)
          (else
            (Variables|Default|SetDoorOpenBack false)))
        (elif (Collision|IsOverlappingActor (Variables|Default|GetFrontSide) Interactor :!class /Script/Engine.PrimitiveComponent)
          (Variables|Default|SetDoorOpenFront true)
          (elif (Collision|IsOverlappingActor (Variables|Default|GetBackSide) Interactor :!class /Script/Engine.PrimitiveComponent)
            (Variables|Default|SetDoorOpenBack true)))))))

(event Custom|Open%20Back
  (if (Variables|Default|GetDoorOpenBack)
    (bind _doormovement (Timeline|DoorAnimation ReverseFromEnd)
      (:Update
        (Transformation|SetRelativeRotation (Variables|Default|GetDoorBody) (Math|Rotator|Lerp(Rotator) (Variables|Default|GetRearRotation) "0, 0, 0" _doormovement) false false)))
    (else
      (Timeline|DoorAnimation PlayFromStart))))