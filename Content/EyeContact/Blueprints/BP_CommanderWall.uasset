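; BP_CommanderWall is a temporary wall that stops human VIPs while they overlap it and resumes them when they leave.
; BuildWall makes the material fully opaque, raises the wall from zero height to its original Z scale with a timeline, and starts a timer for the given duration.
; When the timer fires, ServerDestroyWall destroys the actor.
; SetOpacity can also set a translucent alpha, though BuildWall only uses the opaque state.
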(event Custom|BuildWall
  (params (Duration :type Float%20%28single-precision%29))
  (bind _originalscale (Variables|Default|GetOriginalScale))
  (bind _originalscale_2 (Variables|Default|GetOriginalScale))
  (Transformation|SetActorScale3D (Math|Vector|MakeVector (.x _originalscale) (.y _originalscale) 0.0))
  (CallFunction|SetOpacity true)
  (Utilities|Time|SetTimerbyEvent (delegate Custom|ServerDestroyWall) Duration)
  (bind _floattrack (Timeline|RaiseWallTimeLine PlayFromStart)
    (:Update
      (Transformation|SetActorScale3D (Math|Vector|MakeVector (.x _originalscale_2) (.y _originalscale_2) (* _floattrack (.z _originalscale_2)))))))

(event Custom|ServerDestroyWall
  (Actor|DestroyActor))

(event EventBeginPlay
  (Variables|Default|SetOriginalScale (Transformation|GetActorScale3D)))

(event Collision|EventActorBeginOverlap
  (params (OtherActor :type Actor%20Object%20Reference))
  (bind _asbp_human_vip (Utilities|Casting|CastToBP_HumanVIP OtherActor))
  (Default|ServerStopVIP _asbp_human_vip))

(event Collision|EventActorEndOverlap
  (params (OtherActor :type Actor%20Object%20Reference))
  (bind _asbp_human_vip (Utilities|Casting|CastToBP_HumanVIP OtherActor))
  (Default|ServerResumeVIP _asbp_human_vip))

(fn ConstructionScript)

(fn SetOpacity
  (params (ShouldOpaque :type Boolean))
  (bind _wallmesh (Variables|Default|GetWallMesh))
  (if ShouldOpaque
    (Rendering|Material|SetScalarParameterValueonMaterials _wallmesh "Alpha" 1.0)
    (else
      (Rendering|Material|SetScalarParameterValueonMaterials _wallmesh "Alpha" 0.75))))