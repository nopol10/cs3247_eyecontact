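; Co-op monster that chases the Killer or Spotter player once a human enters its activation zone, freezing while seen.
; The server picks the target by TargetType, moves toward it and, within range, requests a delayed kill through the player controller.
; When a Spotter looks at it, the tag replicates and fades it in for the Killer via a dynamic material.
; Replicated model selection configures both meshes; death swaps to the destructible with blood spray.
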(event OnComponentBeginOverlap(ActivationZone)
  (params (OverlappedComponent :type Primitive%20Component%20Object%20Reference) (OtherActor :type Actor%20Object%20Reference) (OtherComp :type Primitive%20Component%20Object%20Reference) (OtherBodyIndex :type Integer) (bFromSweep :type Boolean) (SweepResult :type Hit%20Result%20Structure%20%28by%20ref%29))
  (Networking|SwitchHasAuthority
    (:Authority
      (Utilities|Casting|CastToHumanPlayer OtherActor)
      (Variables|Default|SetIsActivated true))))

(event Custom|OnMonsterDeath
  (bind _returnvalue (Transformation|GetActorLocation))
  (bind _destructible (Variables|Default|GetDestructible))
  ;[1 1 1] OnMonsterDeath
  (Variables|Default|SetisDead true)
  (Utilities|FlowControl|Sequence
    (:then_0
      ;[1 1 1] Spray blood?
      (Effects|SpawnEmitteratLocation "/Game/EyeContact/Particles/BloodSpray.BloodSpray" (Transformation|GetActorLocation)))
    (:then_1
      (Rendering|SetVisibility (Variables|Default|GetThirdPerson) false false)
      (Rendering|SetVisibility _destructible true false)
      (Game|Damage|ApplyDamage _destructible 1e+01 _returnvalue (- "0, 0, 0" _returnvalue) 1e+01)
      (Utilities|FlowControl|Delay 2.0)
      (Actor|DestroyActor))))

(event Custom|RevealMonster
  (Variables|Default|SetIsTagged true))

(event Custom|FadeInMonster
  (bind _alpha (Timeline|FadeTime Play)
    (:Update
      (Rendering|Material|SetScalarParameterValue (Variables|Default|GetDMI) "Alpha" _alpha :!class /Script/Engine.MaterialInstanceDynamic))))

(event Custom|ServerTryKillPlayer
  (params (Actor :type Actor%20Object%20Reference))
  (if (not (Variables|Default|GetisDead))
    (Utilities|FlowControl|Delay (Variables|Default|GetKillDelay))
    (bind _asbp_eye_contact_controller (Utilities|Casting|CastToBP_EyeContactController (Game|GetPlayerController 0)))
    ;[1 1 1] REPLACE WITH KILL PLAYER CODE
    (Default|ServerKillCoopPlayer _asbp_eye_contact_controller Actor self)
    (Variables|Default|SetIsActivated false)))

(event Custom|Seen
  (params (Id :type Integer))
  (bind _violaterids (Variables|Default|GetViolaterIds))
  ;[1 1 1] Seen and Hidden
  (Utilities|Array|AddUnique _violaterids Id)
  (if (> (Utilities|Array|Length _violaterids) 0)
    (Variables|Default|SetisSeen true)
    (Components|Movement|StopMovementImmediately (Variables|Character|GetCharacterMovement))))

(event Custom|Hidden
  (params (Id :type Integer))
  (bind _violaterids (Variables|Default|GetViolaterIds))
  ;[1 1 1] Seen and Hidden
  (Utilities|Array|RemoveItem _violaterids Id)
  (if (== (Utilities|Array|Length _violaterids) 0)
    (Variables|Default|SetisSeen false)))

(event Custom|Move
  (params (Target :type Actor%20Object%20Reference))
  (if (not (Variables|Default|GetisDead))
    (AI|Navigation|SimpleMovetoActor (Pawn|GetController) Target)))

(event EventLookedat
  (params (Looker :type Actor%20Object%20Reference) (ImpactPoint :type Vector :default "0, 0, 0"))
  (bind _asbp_coop_human_spotter (Utilities|Casting|CastToBP_CoopHumanSpotter Looker))
  (bind _asbp_eye_contact_controller (Utilities|Casting|CastToBP_EyeContactController (Pawn|GetController _asbp_coop_human_spotter)))
  (Default|RevealMonster _asbp_eye_contact_controller self))

(event EventTick
  (params (DeltaSeconds :type Float%20%28single-precision%29))
  (if (not (Variables|Default|GetisDead))
    (Networking|SwitchHasAuthority
      (:Authority
        (if (Variables|Default|GetIsActivated)
          (if (not (Variables|Default|GetisSeen))
            (bind _target (CallFunction|GetTarget))
            (Utilities|IsValid _target
              (:Is%20Valid
                (CallFunction|Move _target)
                (if (Math|Vector|Equal(Vector) (Transformation|GetActorLocation _target) (Transformation|GetActorLocation) 1e+02)
                  (Utilities|FlowControl|DoOnce false :!label _label
                    (:Completed
                      (CallFunction|ServerTryKillPlayer)))
                  (else
                    (goto _label Reset)))))))))))

(event EventBeginPlay
  (bind _thirdperson (Variables|Default|GetThirdPerson))
  (Utilities|FlowControl|Sequence
    (:then_0
      (Networking|SwitchHasAuthority
        (:Authority
          (bind _asbp_eye_contact_game_state (Utilities|Casting|CastToBP_EyeContactGameState (Game|GetGameState)))
          (Variables|Default|SetECGameState _asbp_eye_contact_game_state)
          (Utilities|Array|Add (Variables|/Game/EyeContact/Blueprints/BP_EyeContactGameState.BP_EyeContactGameState_C|GetMonsterPlayers _asbp_eye_contact_game_state) self)
          (CallFunction|InitModel))))
    (:then_1
      (bind _returnvalue (Rendering|Material|CreateDynamicMaterialInstance _thirdperson 0 (Utilities|Array|Get(acopy) (Rendering|Material|GetMaterials _thirdperson)) :!class /Script/Engine.PrimitiveComponent))
      (Variables|Default|SetDMI _returnvalue))))

(fn ConstructionScript)

(fn GetRandomModel
  (bind _possiblemodels (Variables|Default|GetPossibleModels))
  (bind _returnvalue (Utilities|Array|LastIndex _possiblemodels))
  (bind _returnvalue_2 (Math|Random|RandomIntegerinRange 0 _returnvalue))
  (return (Utilities|Array|Get(acopy) _possiblemodels _returnvalue_2) (Utilities|Enum|ByteToEnumMonsterActors (Math|Conversions|ToByte(Integer) _returnvalue_2))))

(fn OnRepIsTagged
  (CallFunction|SetVisibility true)
  (Utilities|Casting|CastToBP_CoopHumanKiller (Pawn|GetControlledPawn (Game|GetPlayerController 0)))
  (CallFunction|FadeinMonster))

(fn GetTarget
  (bind _self self)
  (bind _ecgamestate (Variables|Default|GetECGameState))
  (bind _returnvalue (Transformation|GetActorLocation _self))
  (bind _coopkiller (Variables|/Game/EyeContact/Blueprints/BP_EyeContactGameState.BP_EyeContactGameState_C|GetCoopKiller _ecgamestate))
  (bind _coopspotter (Variables|/Game/EyeContact/Blueprints/BP_EyeContactGameState.BP_EyeContactGameState_C|GetCoopSpotter _ecgamestate))
  (bind _returnvalue_2 (Transformation|GetActorLocation _coopspotter))
  (bind _returnvalue_3 (Transformation|GetActorLocation _coopkiller))
  (bind _distance (CallFunction|DistanceBetweenPoints _returnvalue _returnvalue_2))
  (bind _distance_2 (CallFunction|DistanceBetweenPoints _returnvalue_3 _returnvalue))
  (bind _returnvalue_4 (> _distance_2 _distance))
  (switch Utilities|FlowControl|Switch|SwitchonEMonsterTarget (Variables|Default|GetTargetType)
    (:NewEnumerator0
      (return _coopkiller))
    (:NewEnumerator1
      (return _coopspotter))
    (:NewEnumerator2
      (if _returnvalue_4
        (return _coopspotter)
        (else
          (return _coopkiller))))
    (:NewEnumerator3
      (if _returnvalue_4
        (return _coopkiller)
        (else
          (return _coopspotter))))))

(fn SetVisibility
  (params (Visible :type Boolean))
  (Rendering|SetVisibility (Variables|Character|GetMesh) Visible false))

(fn OnRepIsDead)

(fn InitModel
  (Variables|Default|SetCurrentModel (Utilities|Array|Get(acopy) (Variables|Default|GetPossibleModels) (Math|Conversions|ToInteger(Byte) (Variables|Default|GetModelEnum)))))

(fn OnRepCurrentModel
  (bind _currentmodel (Variables|Default|GetCurrentModel))
  (bind _destructible (Variables|Default|GetDestructible))
  (bind _thirdperson (Variables|Default|GetThirdPerson))
  (bind _modelscales (Variables|Default|GetModelScales))
  (bind _possiblemodels (Variables|Default|GetPossibleModels))
  (bind _modelrotations (Variables|Default|GetModelRotations))
  (bind _returnvalue (Utilities|Array|FindItem _possiblemodels _currentmodel))
  (bind _item (Utilities|Array|Get(acopy) _modelscales _returnvalue))
  (bind _item_2 (Utilities|Array|Get(acopy) _modelrotations _returnvalue))
  (Components|StaticMesh|SetStaticMesh _thirdperson _currentmodel)
  (Transformation|SetWorldScale3D _thirdperson (Math|Vector|MakeVector _item _item _item))
  (Transformation|AddWorldRotation (Variables|Default|GetThirdPerson) (Math|Rotator|MakeRotator 0.0 0.0 _item_2) false false)
  (Class|DestructibleComponent|SetDestructibleMesh _destructible (Utilities|Array|Get(acopy) (Variables|Default|GetDestructibleMeshes) _returnvalue))
  (Transformation|AddWorldRotation _destructible (Math|Rotator|MakeRotator 0.0 0.0 _item_2) false false)
  (Transformation|SetWorldScale3D _destructible (Math|Vector|MakeVector _item _item _item))
  (Rendering|SetVisibility _destructible false false)
  (Collision|SetCollisionEnabled _destructible "NoCollision"))