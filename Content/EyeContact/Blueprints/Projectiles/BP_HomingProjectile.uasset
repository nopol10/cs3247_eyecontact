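; Homing projectile actor that flies toward a human or monster player and carries a configurable particle effect.
; SetTarget points the projectile movement's homing at the target's capsule component.
; When the Cube overlaps that target, it stops the particles, fires OnReachTarget and destroys itself after a short delay.
; The particle template is set through SetParticleClass and reapplied in the ParticleClass RepNotify for replication.
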(event OnComponentBeginOverlap(Cube)
  (params (OverlappedComponent :type Primitive%20Component%20Object%20Reference) (OtherActor :type Actor%20Object%20Reference) (OtherComp :type Primitive%20Component%20Object%20Reference) (OtherBodyIndex :type Integer) (bFromSweep :type Boolean) (SweepResult :type Hit%20Result%20Structure%20%28by%20ref%29))
  (bind _targetactor (Variables|Default|GetTargetActor))
  (Utilities|IsValid _targetactor
    (:Is%20Valid
      (if (== OtherActor _targetactor)
        (Components|Activation|Deactivate (Variables|Default|GetParticleSystem))
        (Default|CallOnReachTarget OtherActor)
        (Utilities|FlowControl|Delay 3.0)
        (Actor|DestroyActor)))))

(event Custom|SetTarget
  (params (TargetActor :type Actor%20Object%20Reference))
  (bind _projectilemovement (Variables|Default|GetProjectileMovement))
  (bind _output_get (Variables|Default|SetTargetActor TargetActor))
  (bind _asbp_human_player (Utilities|Casting|CastToBP_HumanPlayer _output_get)
    (:then
      (Variables|/Script/Engine.ProjectileMovementComponent|SetHomingTargetComponent _projectilemovement (Variables|/Script/Engine.Character|GetCapsuleComponent _asbp_human_player)))
    (:CastFailed
      (bind _asbp_monster_player (Utilities|Casting|CastToBP_MonsterPlayer _output_get))
      (Variables|/Script/Engine.ProjectileMovementComponent|SetHomingTargetComponent _projectilemovement (Variables|/Script/Engine.Character|GetCapsuleComponent _asbp_monster_player)))))

(event EventBeginPlay)

(event Collision|EventActorBeginOverlap
  (params (OtherActor :type Actor%20Object%20Reference)))

(event EventTick
  (params (DeltaSeconds :type Float%20%28single-precision%29)))

(fn ConstructionScript)

(fn SetParticleClass
  (params (ParticleClass :type Particle%20System%20Object%20Reference))
  (bind _output_get (Variables|Default|SetParticleClass ParticleClass))
  (Effects|Components|ParticleSystem|SetTemplate (Variables|Default|GetParticleSystem) _output_get))

(fn OnRepParticleClass
  (Effects|Components|ParticleSystem|SetTemplate (Variables|Default|GetParticleSystem) (Variables|Default|GetParticleClass)))