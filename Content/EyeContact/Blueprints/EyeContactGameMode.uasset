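; Game mode for the Eye Contact humans-versus-monsters match, choosing spawns and pawns by team and handling the end of the game.
; Each controller's team selects a matching Eye Contact player start and either the human or monster pawn, defaulting to human.
; Either win event stops the game, has every controller show win or lose text, then after a delay resets state and team ID lists and server-travels to team select.
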(event Custom|HumansWin
  (bind _asbp_eye_contact_game_state (Utilities|Casting|CastToBP_EyeContactGameState (Game|GetGameState)))
  (Variables|/Game/EyeContact/Blueprints/BP_EyeContactGameState.BP_EyeContactGameState_C|SetGameIsOngoing _asbp_eye_contact_game_state false)
  (bind _outactors (Actor|GetAllActorsOfClass "/Game/EyeContact/Blueprints/BP_EyeContactController.BP_EyeContactController_C"))
  (for _array_element _outactors
    (Default|SpawnHumansWinText _array_element))
  (Utilities|FlowControl|Delay 3.0)
  (CallFunction|ResetGameStatus)
  (Development|ExecuteConsoleCommand "servertravel EC_TeamSelect"))

(event Custom|MonstersWin
  (bind _asbp_eye_contact_game_state (Utilities|Casting|CastToBP_EyeContactGameState (Game|GetGameState)))
  (Variables|/Game/EyeContact/Blueprints/BP_EyeContactGameState.BP_EyeContactGameState_C|SetGameIsOngoing _asbp_eye_contact_game_state false)
  (bind _outactors (Actor|GetAllActorsOfClass "/Game/EyeContact/Blueprints/BP_EyeContactController.BP_EyeContactController_C"))
  (for _array_element _outactors
    (Default|SpawnHumansLoseText _array_element))
  (Utilities|FlowControl|Delay 3.0)
  (CallFunction|ResetGameStatus)
  (Development|ExecuteConsoleCommand "servertravel EC_TeamSelect"))

(event EventBeginPlay)

(event EventTick
  (params (DeltaSeconds :type Float%20%28single-precision%29)))

(event EventPostLogin
  (params (NewPlayer :type Player%20Controller%20Object%20Reference)))

(fn ConstructionScript)

(fn GetPlayerTeam
  (params (PlayerId :type Integer))
  (bind _asbp_eye_contact_game_instance (Utilities|Casting|CastToBP_EyeContactGameInstance (Game|GetGameInstance))
    (:then
      (if (< (Utilities|Array|FindItem (Variables|/Game/EyeContact/Blueprints/BP_EyeContactGameInstance.BP_EyeContactGameInstance_C|GetHumanPlayerIds _asbp_eye_contact_game_instance) PlayerId) 0)
        (if (< (Utilities|Array|FindItem (Variables|/Game/EyeContact/Blueprints/BP_EyeContactGameInstance.BP_EyeContactGameInstance_C|GetMonsterPlayerIds _asbp_eye_contact_game_instance) PlayerId) 0)
          (return "NewEnumerator2")
          (else
            (return "NewEnumerator1")))
        (else
          (return "NewEnumerator0"))))
    (:CastFailed
      (return "NewEnumerator2"))))

(fn ChoosePlayerStart
  (params (Player :type Controller%20Object%20Reference))
  (bind _asbp_eye_contact_controller (Utilities|Casting|CastToBP_EyeContactController Player)
    (:then
      (bind _selectiontype (Default|GetPlayerTeam _asbp_eye_contact_controller (Variables|/Script/Engine.PlayerState|GetPlayerId (Variables|/Script/Engine.Controller|GetPlayerState _asbp_eye_contact_controller))))
      (Development|PrintString (Utilities|String|Append (Utilities|String|ToString(Integer) (Variables|/Script/Engine.PlayerState|GetPlayerId (Variables|/Script/Engine.Controller|GetPlayerState _asbp_eye_contact_controller))) " spawning as " (Utilities|String|EnumtoString _selectiontype)) true true "(R=0.000000,G=0.660000,B=1.000000,A=1.000000)" 15.0)
      (bind _outactors (Actor|GetAllActorsOfClass "/Game/EyeContact/Blueprints/BP_EyeContactPlayerStart.BP_EyeContactPlayerStart_C"))
      (for _array_element _outactors
        (if (Utilities|Enum|Equal(Enum) _selectiontype (Variables|/Game/EyeContact/Blueprints/BP_EyeContactPlayerStart.BP_EyeContactPlayerStart_C|GetPlayerType _array_element))
          (bind _spawnposition (Default|GetRandomSpawnPosition _array_element))
          (return _spawnposition)))
      (bind _spawnposition_2 (Default|GetRandomSpawnPosition (Utilities|Array|Get(acopy) _outactors)))
      (return _spawnposition_2))
    (:CastFailed
      ;[1 1 1] No BP_EyeContactPlayerStart found
      (bind _outactors_2 (Actor|GetAllActorsOfClass "/Script/Engine.PlayerStart"))
      (return (Utilities|Array|Get(acopy) _outactors_2)))))

(fn GetDefaultPawnClassforController
  (params (InController :type Controller%20Object%20Reference))
  (bind _asbp_eye_contact_controller (Utilities|Casting|CastToBP_EyeContactController InController)
    (:then
      (bind _selectiontype (Default|GetPlayerTeam _asbp_eye_contact_controller (Variables|/Script/Engine.PlayerState|GetPlayerId (Variables|/Script/Engine.Controller|GetPlayerState _asbp_eye_contact_controller))))
      (switch Utilities|FlowControl|Switch|SwitchonEPlayerType _selectiontype
        (:NewEnumerator0
          (return "/Game/EyeContact/Blueprints/BP_HumanPlayer.BP_HumanPlayer_C"))
        (:NewEnumerator1
          (return "/Game/EyeContact/Blueprints/BP_MonsterPlayer.BP_MonsterPlayer_C"))
        (:NewEnumerator2
          _)))
    (:CastFailed
      _))
  (return "/Game/EyeContact/Blueprints/BP_HumanPlayer.BP_HumanPlayer_C"))

(fn ResetGameStatus
  (Variables|Default|SetHumansHaveGoal false)
  (bind _asbp_eye_contact_game_state (Utilities|Casting|CastToBP_EyeContactGameState (Game|GetGameState)))
  (Variables|/Game/EyeContact/Blueprints/BP_EyeContactGameState.BP_EyeContactGameState_C|SetGameIsOngoing _asbp_eye_contact_game_state true)
  (Utilities|Array|Clear (Variables|/Game/EyeContact/Blueprints/BP_EyeContactGameState.BP_EyeContactGameState_C|GetMonsterPlayers _asbp_eye_contact_game_state))
  (bind _asbp_eye_contact_game_instance (Utilities|Casting|CastToBP_EyeContactGameInstance (Game|GetGameInstance)))
  (Utilities|Array|Clear (Variables|/Game/EyeContact/Blueprints/BP_EyeContactGameInstance.BP_EyeContactGameInstance_C|GetHumanPlayerIds _asbp_eye_contact_game_instance))
  (Utilities|Array|Clear (Variables|/Game/EyeContact/Blueprints/BP_EyeContactGameInstance.BP_EyeContactGameInstance_C|GetMonsterPlayerIds _asbp_eye_contact_game_instance)))