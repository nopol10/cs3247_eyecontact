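; EyeContactTeamSelectMode is the game mode for team selection, tracking connected players and giving each a selection indicator.
; PostLogin adds the controller to PlayerControllers and spawns a BP_SelectingIndicator below the first BP_SpawnLocation, stepped down vertically by the new array index.
; OnLogout removes the controller from the array but leaves its indicator in place.
; GetPlayerCount returns the array's length.
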(event EventBeginPlay
  (bind _outactors (Actor|GetAllActorsOfClass "/Game/EyeContact/Blueprints/TeamSelect/BP_SpawnLocation.BP_SpawnLocation_C"))
  (Variables|Default|SetSpawnLocation (Utilities|Array|Get(acopy) _outactors))
  (Development|PrintString "TeamSelectGameMode begin"))

(event EventTick
  (params (DeltaSeconds :type Float%20%28single-precision%29)))

(event EventPostLogin
  (params (NewPlayer :type Player%20Controller%20Object%20Reference))
  (bind _outactors (Actor|GetAllActorsOfClass "/Game/EyeContact/Blueprints/TeamSelect/BP_SpawnLocation.BP_SpawnLocation_C"))
  (Variables|Default|SetSpawnLocation (Utilities|Array|Get(acopy) _outactors))
  (Development|PrintString "Post login loool")
  (bind _returnvalue (Utilities|Array|Add (Variables|Default|GetPlayerControllers) NewPlayer))
  (Game|SpawnActorfromClass "/Game/EyeContact/Blueprints/TeamSelect/BP_SelectingIndicator.BP_SelectingIndicator_C" (Math|Conversions|ToTransform(Vector) (+ (Transformation|GetActorLocation (Variables|Default|GetSpawnLocation)) (* "0, 0,-120.000000" _returnvalue))) "Undefined" 0 0))

(event EventOnLogout
  (params (ExitingController :type Controller%20Object%20Reference))
  (Development|PrintString "Player left the game")
  (bind _returnvalue (Utilities|Casting|CastToPlayerController ExitingController))
  (Utilities|Array|RemoveItem (Variables|Default|GetPlayerControllers) _returnvalue))

(fn ConstructionScript)

(fn GetPlayerCount
  (return (Utilities|Array|Length (Variables|Default|GetPlayerControllers))))