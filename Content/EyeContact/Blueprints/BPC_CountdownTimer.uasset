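; BPC_CountdownTimer is an actor component that shows the EyeContact game state's remaining time as a countdown on its owner.
; While enabled, each tick copies RemainingTime from BP_EyeContactGameState rather than counting down locally.
; It writes the prettified time to every owner TextRender component tagged CountdownText.
; When time reaches zero, it fires OnTimerEnd and disables itself.
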(event EventBeginPlay)

(event EventTick
  (params (DeltaSeconds :type Float%20%28single-precision%29))
  (if (Variables|Default|GetCountdownEnabled)
    (bind _asbp_eye_contact_game_state (Utilities|Casting|CastToBP_EyeContactGameState (Game|GetGameState)))
    (bind _output_get (Variables|Default|SetCountdownTime (Variables|/Game/EyeContact/Blueprints/BP_EyeContactGameState.BP_EyeContactGameState_C|GetRemainingTime _asbp_eye_contact_game_state)))
    (CallFunction|UpdateTimer)
    (if (<= _output_get 0.0)
      (Default|CallOnTimerEnd)
      (Variables|Default|SetCountdownEnabled false))))

(fn UpdateTimer
  (bind _resulttime (CallFunction|PrettifyTime (Variables|Default|GetCountdownTime)))
  (for _array_element (Actor|GetComponentsbyTag (Components|GetOwner) "/Script/Engine.TextRenderComponent" "CountdownText")
    (Rendering|Components|TextRender|SetText _array_element (Utilities|Text|ToText(String) _resulttime))))