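; BP_MonsterAttacker is the attacker monster, with two input-driven skills: spawning illusions and teleporting.
; Skill1 spawns a BP_MonsterIllusion behind the monster, gated by a cooldown and an illusion count limit.
; Skill2 teleports to the oldest illusion and destroys it, or jumps along the camera's forward vector if none exist.
; Tick counts down both cooldowns, though Skill2 never checks its own before firing.
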(event Custom|SpawnIllusion
  (bind _thirdperson (Variables|Default|GetThirdPerson))
  (bind _returnvalue (Transformation|GetWorldTransform _thirdperson))
  ;[1 1 1] Spawn Illusion Skill
  (bind _returnvalue_2 (Game|SpawnActorfromClass "/Game/EyeContact/Blueprints/BP_MonsterIllusion.BP_MonsterIllusion_C" (Math|Transform|MakeTransform (- (.location _returnvalue) (* (Math|Vector|GetForwardVector (Variables|Default|GetCamera)) 200)) (.rotation _returnvalue) "1.000000,1.000000,1.000000") "AdjustIfPossibleButAlwaysSpawn" 0 self))
  (Utilities|Array|Add (Variables|Default|GetIllusions) _returnvalue_2)
  (Variables|Default|SetSpawnIlluRemainingCd (Variables|Default|GetSpawnIlluCooldown)))

(event Custom|TeleportSkill
  (bind _camera (Variables|Default|GetCamera))
  (bind _illusions (Variables|Default|GetIllusions))
  (bind _item (Utilities|Array|Get(acopy) _illusions))
  (if (> (Utilities|Array|Length (Variables|Default|GetIllusions)) 0)
    (bind _output_get (Variables|Default|SetIlluLocation (Transformation|GetActorLocation _item)))
    (bind _output_get_2 (Variables|Default|SetIlluRotation (Transformation|GetActorRotation _item)))
    (Actor|DestroyActor _item)
    (Utilities|Array|RemoveIndex _illusions)
    (bind _returnvalue (Transformation|Teleport _output_get _output_get_2))
    (Development|PrintString (Utilities|String|ToString(Boolean) _returnvalue))
    (else
      (Transformation|Teleport (+ (* (Math|Vector|GetForwardVector _camera) 500) (Transformation|GetActorLocation)) (Transformation|GetWorldRotation _camera))))
  (Variables|Default|SetTeleportRemainingCd (Variables|Default|GetTeleportSkillCooldown)))

(event EventBeginPlay
  (|CallParentFunction)
  (Development|PrintString "Is attacker"))

(event Collision|EventActorBeginOverlap
  (params (OtherActor :type Actor%20Object%20Reference)))

(event EventTick
  (params (DeltaSeconds :type Float%20%28single-precision%29))
  (|CallParentFunction 0.0)
  (CallFunction|UpdateSkillTimers DeltaSeconds))

(event Input|ActionEvents|InputActionSkill1
  (params (Key :type Key%20Structure :default "AnyKey"))
  ;[1 1 1] Spawn Illusion Skill
  (:Pressed
    (if (<= (Variables|Default|GetSpawnIlluRemainingCd) 0.0)
      (if (>= (Variables|Default|GetMaxIllusions) (Utilities|Array|Length (Variables|Default|GetIllusions)))
        (CallFunction|SpawnIllusion)
        (else
          (Development|PrintString "Max illusions reached!"))))))

(event Input|ActionEvents|InputActionSkill2
  (params (Key :type Key%20Structure :default "AnyKey"))
  (:Pressed
    (CallFunction|TeleportSkill)))

(fn ConstructionScript
  (|CallParentFunction))

(fn UpdateSkillTimers
  (params (DeltaSeconds :type Float%20%28single-precision%29))
  (if (> (Variables|Default|GetSpawnIlluRemainingCd) 0.0)
    (bind _output_get (Variables|Default|SetSpawnIlluRemainingCd (- (Variables|Default|GetSpawnIlluRemainingCd) DeltaSeconds)))
    (if (not (> _output_get 0.0))
      (Development|PrintString "Spawn Illusion available!")
      (if (> (Variables|Default|GetTeleportRemainingCd) 0.0) :!label _label
        (bind _output_get_2 (Variables|Default|SetTeleportRemainingCd (- (Variables|Default|GetTeleportRemainingCd) DeltaSeconds)))
        (if (not (> _output_get_2 0.0))
          (Development|PrintString "Teleport available"))))
    (else
      (goto _label))))