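; A Blueprint function library of small shared helpers for the EyeContact game.
; It wraps a key-array membership check, returns the first BP_MenuVariableHolder actor in the level, and rewinds and stops a timeline without firing events.
; Vector helpers turn a scene component's X axis toward a target actor after validity checks and return the angle in degrees between two vectors.
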(fn ContainsKey
  (params (KeyArray :type Array%20of%20Key%20Structures) (InKey :type Key%20Structure :default "AnyKey"))
  (return (Utilities|Array|ContainsItem KeyArray InKey)))

(fn GetMenuVariable
  (bind _outactors (Actor|GetAllActorsOfClass 0 "/Game/EyeContact/Blueprints/Lobby/BP_MenuVariableHolder.BP_MenuVariableHolder_C"))
  (return (Utilities|Array|Get(acopy) _outactors)))

(fn ResetTimeline
  (params (Timeline :type Timeline%20Component%20Object%20Reference))
  (Components|Timeline|SetPlaybackPosition Timeline 0.0 false true)
  (Audio|Components|Audio|Stop Timeline))

(fn FaceObject
  (params (Source :type Scene%20Component%20Object%20Reference) (Target :type Actor%20Object%20Reference))
  (if (and (Utilities|IsValid Target) (Utilities|IsValid Source))
    (Transformation|SetWorldRotation Source (Math|Conversions|RotationFromXVector (Math|Vector|RotateVector (Math|Vector|Normalize (* (- (Transformation|GetActorLocation Target) (Transformation|GetWorldLocation Source)) "1.000000,1.000000,1.000000")) "0, 0, 0")) false false)))

(fn AngleBetweenTwoVectors
  (params (u :type Vector) (V :type Vector))
  (return (Class|KismetMathLibrary|DegAcos (Math|Vector|DotProduct (Math|Vector|Normalize u) (Math|Vector|Normalize V)))))