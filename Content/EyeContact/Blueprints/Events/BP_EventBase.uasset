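; BP_EventBase is a base actor for trigger events that fire when a human co-op character enters its box.
; The overlap runs only on the authority and uses IsHuman to accept BP_CoopHumanKiller or BP_CoopHumanSpotter actors.
; While TriggeredCount is below MaxTriggerCount, it calls RunTriggerEvent and increments the count.
; RunTriggerEvent is empty here, serving as the hook for the event's actual behavior.
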(event OnComponentBeginOverlap(Box)
  (params (OverlappedComponent :type Primitive%20Component%20Object%20Reference) (OtherActor :type Actor%20Object%20Reference) (OtherComp :type Primitive%20Component%20Object%20Reference) (OtherBodyIndex :type Integer) (bFromSweep :type Boolean) (SweepResult :type Hit%20Result%20Structure%20%28by%20ref%29))
  (Networking|SwitchHasAuthority
    (:Authority
      (bind _ishuman (CallFunction|IsHuman OtherActor))
      (if (and _ishuman (< (Variables|Default|GetTriggeredCount) (Variables|Default|GetMaxTriggerCount)))
        (CallFunction|RunTriggerEvent)
        (Math|Integer|IncrementInt (Variables|Default|GetTriggeredCount))))))

(event Custom|RunTriggerEvent)

(event EventBeginPlay)

(event Collision|EventActorBeginOverlap
  (params (OtherActor :type Actor%20Object%20Reference)))

(event EventTick
  (params (DeltaSeconds :type Float%20%28single-precision%29)))

(fn ConstructionScript)

(fn IsHuman
  (params (Actor :type Actor%20Object%20Reference))
  (Utilities|Casting|CastToBP_CoopHumanKiller Actor
    (:then
      _)
    (:CastFailed
      (Utilities|Casting|CastToBP_CoopHumanSpotter Actor
        (:then
          _)
        (:CastFailed
          (return false)))))
  (return true))