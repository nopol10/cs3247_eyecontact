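; Player controller for Eye Contact's humans-versus-monsters matches, handling deaths, match-end feedback and team lookup.
; Server kill logic drops a carried goal object, triggers human death and calls MonstersWin on the game mode once all humans are dead.
; Win/lose events attach team-specific text to the pawn, then MoveToEndPoint disables gravity; its teleport nodes are unwired.
; It also looks up teams in the game instance, plays goal-pickup roars and switches resolution quality.
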(event Custom|KillHuman
  (params (TargetPlayer :type BP%20Human%20Player%20Object%20Reference))
  (CallFunction|ServerKillPlayer TargetPlayer))

(event Custom|SpawnEmitter
  (params (Particle :type Particle%20System%20Object%20Reference) (Location :type Vector))
  (Effects|SpawnEmitteratLocation Particle Location))

(event Custom|ServerKillPlayer
  (params (TargetPlayer :type BP%20Human%20Player%20Object%20Reference))
  ;[1 1 1] Kill a given player - server internal call
  (if (not (Variables|/Game/EyeContact/Blueprints/BP_HumanPlayer.BP_HumanPlayer_C|GetIsDead TargetPlayer))
    (bind _aseye_contact_game_mode (Utilities|Casting|CastToEyeContactGameMode (Game|GetGameMode)))
    (Variables|/Game/EyeContact/Blueprints/BP_HumanPlayer.BP_HumanPlayer_C|SetIsDead TargetPlayer true)
    (if (Variables|/Game/EyeContact/Blueprints/BP_HumanPlayer.BP_HumanPlayer_C|GetHasGoalObject TargetPlayer)
      (Game|SpawnActorfromClass "/Game/EyeContact/Blueprints/BP_GoalObject.BP_GoalObject_C" (Math|Conversions|ToTransform(Vector) (Transformation|GetActorLocation TargetPlayer)) "Undefined" 0 0)
      (Variables|/Game/EyeContact/Blueprints/EyeContactGameMode.EyeContactGameMode_C|SetHumansHaveGoal _aseye_contact_game_mode false))
    (Default|OnHumanDeath TargetPlayer)
    (bind _outactors (Actor|GetAllActorsOfClass "/Game/EyeContact/Blueprints/BP_HumanPlayer.BP_HumanPlayer_C"))
    (bind _array_element (Utilities|Array|ForEachLoopwithBreak _outactors)
      (:LoopBody
        (if (not (Variables|/Game/EyeContact/Blueprints/BP_HumanPlayer.BP_HumanPlayer_C|GetIsDead _array_element))
          (Variables|Default|SetAllHumansDead false)))
      (:Completed
        (if (Variables|Default|GetAllHumansDead)
          (Default|MonstersWin _aseye_contact_game_mode) ; For now since we set to 1 human player monsters win when a guy dies
          (else
            (Variables|Default|SetAllHumansDead true)))))))

(event Custom|GoalPickedUp
  ;[1 1 1] On Goal Picked up
  (bind _outactors (Actor|GetAllActorsOfClass "/Game/EyeContact/Blueprints/BP_MonsterPlayer.BP_MonsterPlayer_C"))
  (for _array_element _outactors
    (Audio|PlaySoundatLocation "/Game/EyeContact/Sounds/SC_Roar.SC_Roar" (Transformation|GetActorLocation))
    (Development|PrintString "Monster roar")))

(event Custom|SpawnHumansLoseText
  (bind _returnvalue (Pawn|GetControlledPawn))
  (bind _returnvalue_2 (Game|SpawnActorfromClass "/Game/EyeContact/Blueprints/BP_YouWin.BP_YouWin_C" (Math|Conversions|ToTransform(Vector) (+ (Transformation|GetActorLocation _returnvalue) (* (Transformation|GetActorForwardVector _returnvalue) 3e+02) "0,0,100.000000")) "Undefined" 0 0))
  (Class|Actor|AttachRootComponenttoActor _returnvalue_2 _returnvalue "None" "KeepRelativeOffset" true)
  (Utilities|Casting|CastToBP_HumanPlayer _returnvalue
    (:then
      (Rendering|Components|TextRender|SetText (Variables|/Game/EyeContact/Blueprints/BP_YouWin.BP_YouWin_C|GetWinLoseText _returnvalue_2) (Utilities|Text|ToText(String) (Utilities|String|MakeLiteralString "You Lose"))))
    (:CastFailed
      (Utilities|Casting|CastToBP_MonsterPlayer _returnvalue)
      (Rendering|Components|TextRender|SetText (Variables|/Game/EyeContact/Blueprints/BP_YouWin.BP_YouWin_C|GetWinLoseText _returnvalue_2) (Utilities|Text|ToText(String) (Utilities|String|MakeLiteralString "You Win")))))
  (CallFunction|MovetoEndPoint))

(event Custom|ServerKillMonster
  (params (TargetMonster :type BP%20Monster%20Player%20Object%20Reference))
  (if (not (Variables|/Game/EyeContact/Blueprints/BP_MonsterPlayer.BP_MonsterPlayer_C|GetisDead TargetMonster))
    (Default|OnMonsterDeath TargetMonster)))

(event Custom|SetActorLocationToEnd
  (Transformation|SetActorLocation (Pawn|GetControlledPawn) "9999.000000,9999.000000,9999.000000" false true))

(event Custom|SpawnHumansWinText
  (bind _returnvalue (Pawn|GetControlledPawn))
  (bind _returnvalue_2 (Game|SpawnActorfromClass "/Game/EyeContact/Blueprints/BP_YouWin.BP_YouWin_C" (Math|Conversions|ToTransform(Vector) (+ (Transformation|GetActorLocation _returnvalue) (* (Transformation|GetActorForwardVector _returnvalue) 3e+02) "0,0,100.000000")) "Undefined" 0 0))
  (Class|Actor|AttachRootComponenttoActor _returnvalue_2 _returnvalue "None" "KeepRelativeOffset" true)
  (Utilities|Casting|CastToBP_HumanPlayer _returnvalue
    (:then
      (Rendering|Components|TextRender|SetText (Variables|/Game/EyeContact/Blueprints/BP_YouWin.BP_YouWin_C|GetWinLoseText _returnvalue_2) (Utilities|Text|ToText(String) (Utilities|String|MakeLiteralString "You Win"))))
    (:CastFailed
      (Utilities|Casting|CastToBP_MonsterPlayer _returnvalue)
      (Rendering|Components|TextRender|SetText (Variables|/Game/EyeContact/Blueprints/BP_YouWin.BP_YouWin_C|GetWinLoseText _returnvalue_2) (Utilities|Text|ToText(String) (Utilities|String|MakeLiteralString "You Lose")))))
  (CallFunction|MovetoEndPoint))

(event EventBeginPlay
  (Networking|SwitchHasAuthority
    (:Authority
      (CallFunction|GetPlayerTeam (Variables|/Script/Engine.PlayerState|GetPlayerId (Variables|GetPlayerState))))))

(event Input|ActionEvents|InputActionLowQuality
  (params (Key :type Key%20Structure :default "AnyKey"))
  (:Pressed
    (Development|ExecuteConsoleCommand "sg.ResolutionQuality 40")))

(event Input|ActionEvents|InputActionHighQuality
  (params (Key :type Key%20Structure :default "AnyKey"))
  (:Pressed
    (Development|ExecuteConsoleCommand "sg.ResolutionQuality 100")))

(fn ConstructionScript)

(fn GetPlayerTeam
  (params (PlayerId :type Integer))
  (bind _asbp_eye_contact_game_instance (Utilities|Casting|CastToBP_EyeContactGameInstance (Game|GetGameInstance))
    (:then
      (if (< (Utilities|Array|FindItem (Variables|/Game/EyeContact/Blueprints/BP_EyeContactGameInstance.BP_EyeContactGameInstance_C|GetHumanPlayerIds _asbp_eye_contact_game_instance) PlayerId) 0)
        (if (< (Utilities|Array|FindItem (Variables|/Game/EyeContact/Blueprints/BP_EyeContactGameInstance.BP_EyeContactGameInstance_C|GetMonsterPlayerIds _asbp_eye_contact_game_instance) PlayerId) 0)
          (Development|PrintString (Utilities|String|ToString(Integer) (Utilities|Array|Length (Variables|/Game/EyeContact/Blueprints/BP_EyeContactGameInstance.BP_EyeContactGameInstance_C|GetMonsterPlayerIds _asbp_eye_contact_game_instance))))
          (return "NewEnumerator2")
          (else
            (return "NewEnumerator1")))
        (else
          (return "NewEnumerator0"))))
    (:CastFailed
      (Development|PrintString "Game Instrance Not Found")
      (return "NewEnumerator2"))))

(fn MovetoEndPoint
  (bind _returnvalue (Pawn|GetControlledPawn))
  (bind _ascharacter (Utilities|Casting|CastToCharacter _returnvalue))
  (bind _asbp_monster_player (Utilities|Casting|CastToBP_MonsterPlayer _returnvalue)
    (:then
      (Rendering|SetOnlyOwnerSee (Variables|/Game/EyeContact/Blueprints/BP_MonsterPlayer.BP_MonsterPlayer_C|GetThirdPerson _asbp_monster_player) true :!class /Script/Engine.PrimitiveComponent)
      (Class|PrimitiveComponent|SetOwnerNoSee (Variables|/Game/EyeContact/Blueprints/BP_MonsterPlayer.BP_MonsterPlayer_C|GetThirdPerson _asbp_monster_player) true))
    (:CastFailed
      (Utilities|Casting|CastToBP_HumanPlayer _returnvalue)))
  (Physics|SetEnableGravity (Variables|/Script/Engine.Character|GetCapsuleComponent _ascharacter) false))

(fn OnRepPosition
  (Transformation|SetActorLocation (Pawn|GetControlledPawn) (Variables|Default|GetPosition) false true))

(fn IsinGlitchedTeamSelect
  (bind _returnvalue (Game|GetCurrentLevelName true))
  (return (Utilities|Enum|Equal(Enum) _returnvalue "EC_TeamSelect")))

(fn OnRepDeathRotation
  (bind _asbp_human_player (Utilities|Casting|CastToBP_HumanPlayer (Pawn|GetControlledPawn)))
  (Transformation|SetRelativeRotation (Variables|/Script/Engine.Character|GetMesh _asbp_human_player) (Math|Rotator|MakeRotator 0.0 0.0 -9e+01) false false)
  (Development|PrintString (Utilities|String|ToString(Float) 0.0)))