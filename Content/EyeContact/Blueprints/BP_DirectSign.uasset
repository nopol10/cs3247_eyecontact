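; BP_DirectSign is a signpost actor whose Pointer component aims at the active end goal of the EyeContact game.
; UpdateSign, not called within this file, runs on the authority: after a short delay it computes a look-at rotation toward the game state's ActiveEndGoal.
; The result goes into the RepNotify variable Rotation, whose OnRep applies it to the Pointer and prints it for debugging.
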(event Custom|UpdateSign
  (Networking|SwitchHasAuthority
    (:Authority
      (Utilities|FlowControl|Delay 1.0)
      (bind _asbp_eye_contact_game_state (Utilities|Casting|CastToBP_EyeContactGameState (Game|GetGameState)))
      (Variables|Default|SetRotation (Math|Rotator|FindLookatRotation (Transformation|GetWorldLocation (Variables|Default|GetPointer)) (Transformation|GetActorLocation (Variables|/Game/EyeContact/Blueprints/BP_EyeContactGameState.BP_EyeContactGameState_C|GetActiveEndGoal _asbp_eye_contact_game_state)))))))

(event EventBeginPlay)

(event EventActorBeginOverlap
  (params (OtherActor :type Actor%20Object%20Reference)))

(event EventTick
  (params (DeltaSeconds :type Float%20%28single-precision%29)))

(fn ConstructionScript)

(fn OnRepRotation
  (CallFunction|UpdateRotation))

(fn UpdateRotation
  (bind _rotation (Variables|Default|GetRotation))
  (Transformation|SetWorldRotation (Variables|Default|GetPointer) _rotation false false)
  (Development|PrintString (Utilities|String|ToString(Rotator) _rotation)))