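; BP_VIPwaypoints is a waypoint sequence actor, named for a VIP, that hands out route points in order.
; GetNextPoint returns the Waypoints entry at CurrentIndex and advances the index, guarded by HasNextPoint, which checks it against the array length.
; The index never wraps or resets here, so the route is consumed once; the event graph and construction script are empty.
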(event EventBeginPlay)

(event Collision|EventActorBeginOverlap
  (params (OtherActor :type Actor%20Object%20Reference)))

(event EventTick
  (params (DeltaSeconds :type Float%20%28single-precision%29)))

(fn ConstructionScript)

(fn GetNextPoint
  (bind _hasnext (CallFunction|HasNextPoint))
  (if _hasnext
    (bind _output_get (LocalVariables|SetRes (Utilities|Array|Get(acopy) (Variables|Default|GetWaypoints) (Variables|Default|GetCurrentIndex))))
    (Math|Integer|IncrementInt (Variables|Default|GetCurrentIndex)
      (:%20%20
        (return _output_get)))))

(fn HasNextPoint
  (return (< (Variables|Default|GetCurrentIndex) (Utilities|Array|Length (Variables|Default|GetWaypoints)))))