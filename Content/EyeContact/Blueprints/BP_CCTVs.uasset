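; BP_CCTVs holds the list of CCTVs and tracks which one is current.
; Three functions return the current, next or previous entry from the CCTVs array, with next and previous moving a shared index that wraps around at either end.
; It has no active event or construction logic, so the index changes only when next or previous is called.
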(event EventBeginPlay)

(event Collision|EventActorBeginOverlap
  (params (OtherActor :type Actor%20Object%20Reference)))

(event EventTick
  (params (DeltaSeconds :type Float%20%28single-precision%29)))

(fn ConstructionScript)

(fn GetCurrentCCTV
  (return (Utilities|Array|Get(acopy) (Variables|Default|GetCCTVs) (Variables|Default|GetCurrentIndex))))

(fn GetNextCCTV
  (bind _cctvs (Variables|Default|GetCCTVs))
  (bind _result (Math|Integer|IncrementInt (Variables|Default|GetCurrentIndex))
    (:%20%20
      (if (>= _result (Utilities|Array|Length _cctvs))
        (Variables|Default|SetCurrentIndex 0))
      (return (Utilities|Array|Get(acopy) _cctvs (Variables|Default|GetCurrentIndex))))))

(fn GetPrevCCTV
  (bind _cctvs (Variables|Default|GetCCTVs))
  (bind _result (Math|Integer|DecrementInt (Variables|Default|GetCurrentIndex))
    (:%20%20
      (if (< _result 0)
        (Variables|Default|SetCurrentIndex (- (Utilities|Array|Length _cctvs) 1)))
      (return (Utilities|Array|Get(acopy) _cctvs (Variables|Default|GetCurrentIndex))))))