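; BP_HumanVIP is the human VIP character that walks a waypoint route and triggers the monsters' win on reaching its end.
; BeginPlay finds the BP_VIPwaypoints actor, outlines goal-object swords, highlights monsters if the VIP is player pawn 0, then starts moving.
; Movement uses SimpleMoveToActor, with a Tick proximity check behind a DoOnce requesting each next point.
; When no points remain, it calls MonstersWin on the game mode.
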(event Custom|MoveVIP
  (bind _vipwaypoint (Variables|Default|GetVIPWaypoint))
  (bind _hasnext (Default|HasNextPoint _vipwaypoint))
  (if _hasnext
    (bind _wp (Default|GetNextPoint _vipwaypoint))
    (Variables|Default|SetCurrentWpPosition (Transformation|GetActorLocation _wp))
    (AI|Navigation|SimpleMovetoActor (Pawn|GetController) _wp)
    (else
      (CallFunction|ReachEndPoint))))

(event Custom|Outline%20Monsters
  (params (ShouldOutline :type Boolean))
  (if (== (Game|Player|GetPlayerPawn 0) self)
    (bind _outactors (Actor|GetAllActorsOfClass "/Game/EyeContact/Blueprints/BP_MonsterPlayer.BP_MonsterPlayer_C"))
    ;[1 1 1] TODO: OUTLINE HERE (done need to verify)
    (for _array_element _outactors
      (Default|HighlightMonster _array_element))))

(event Custom|ReachEndPoint
  ;[1 1 1] ADD REACH ENDPOINT CODE
  (Development|PrintString "ENDPOINT REACHED!!!")
  (bind _aseye_contact_game_mode (Utilities|Casting|CastToEyeContactGameMode (Game|GetGameMode)))
  (Default|MonstersWin _aseye_contact_game_mode))

(event Custom|Outline%20Swords
  (params (ShouldOutline :type Boolean))
  (bind _outactors (Actor|GetAllActorsOfClass "/Game/EyeContact/Blueprints/BP_GoalObject.BP_GoalObject_C"))
  (for _array_element _outactors
    (Default|ShouldOutlineObject _array_element ShouldOutline self)))

(event EventBeginPlay
  (Development|PrintString "VIP HELLO")
  (|CallParentFunction)
  (CallFunction|DeleteGoalInfo)
  (Variables|Default|SetShouldEnableMovement false)
  (bind _outactors (Actor|GetAllActorsOfClass "/Game/EyeContact/Blueprints/BP_VIPwaypoints.BP_VIPwaypoints_C"))
  (if (> (Utilities|Array|Length _outactors) 0)
    (Variables|Default|SetVIPWaypoint (Utilities|Array|Get(acopy) _outactors))
    (CallFunction|OutlineSwords true)
    (CallFunction|OutlineMonsters true)
    (CallFunction|MoveVIP)))

(event EventTick
  (params (DeltaSeconds :type Float%20%28single-precision%29))
  (|CallParentFunction DeltaSeconds)
  (if (Math|Vector|Equal(Vector) (Variables|Default|GetCurrentWpPosition) (Transformation|GetActorLocation) 1e+02)
    (Utilities|FlowControl|DoOnce false :!label _label
      (:Completed
        (CallFunction|MoveVIP)))
    (else
      (goto _label Reset))))

(fn ConstructionScript)