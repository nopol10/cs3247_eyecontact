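; EyeContactVIP game mode that picks each player's pawn for a Human versus Monster match and uses a separate pawn on the end map.
; Pawn selection matches the player's team and saved class index from the game instance against its class lists.
; Teamless players, an editor-only case, get a random side recorded in the game instance; failed casts fall back to the monster pawn.
; The win-condition check only prints a debug string.
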(event EventBeginPlay
  (|CallParentFunction)
  (Utilities|Casting|CastToBP_HumanPlayer (Game|GetPlayerCharacter 0)))

(event EventCheckWinCondition
  (Development|PrintString "VIP CHecking Win Condition"))

(fn ConstructionScript
  (|CallParentFunction))

(fn GetDefaultPawnClassFinal
  (params (InController :type Controller%20Object%20Reference))
  (Development|PrintString "Using VIP pawn class selection")
  (bind _returnvalue (Game|GetCurrentLevelName true))
  (if (Utilities|Enum|Equal(Enum) _returnvalue "EC_EndMap")
    (return "/Game/EyeContact/Blueprints/BP_EndMapPawn.BP_EndMapPawn_C")
    (else
      (bind _asbp_eye_contact_controller (Utilities|Casting|CastToBP_EyeContactController InController)
        (:then
          (bind _selectiontype (Default|GetPlayerTeam _asbp_eye_contact_controller (Variables|/Script/Engine.PlayerState|GetPlayerId (Variables|/Script/Engine.Controller|GetPlayerState _asbp_eye_contact_controller))))
          (Development|PrintString (Utilities|String|Append (Utilities|String|EnumtoString _selectiontype) (Utilities|String|ToString(Integer) (Variables|/Script/Engine.PlayerState|GetPlayerId (Variables|/Script/Engine.Controller|GetPlayerState _asbp_eye_contact_controller)))) true true "(R=0.000000,G=0.660000,B=1.000000,A=1.000000)" 6.0)
          (bind _asbp_eye_contact_game_instance (Utilities|Casting|CastToBP_EyeContactGameInstance (Game|GetGameInstance))
            (:then
              (for _array_element (Variables|/Game/EyeContact/Blueprints/BP_EyeContactGameInstance.BP_EyeContactGameInstance_C|GetPlayerClassIds _asbp_eye_contact_game_instance)
                (if (== (Variables|/Script/Engine.PlayerState|GetPlayerId (Variables|/Script/Engine.Controller|GetPlayerState _asbp_eye_contact_controller)) (.key _array_element))
                  (LocalVariables|SetSelectedClassIndex (.value _array_element))))
              (switch Utilities|FlowControl|Switch|SwitchonEPlayerType _selectiontype
                (:NewEnumerator0
                  (return (.pawnclass (Utilities|Array|Get(acopy) (Variables|/Game/EyeContact/Blueprints/BP_EyeContactGameInstance.BP_EyeContactGameInstance_C|GetHumanClasses _asbp_eye_contact_game_instance) (LocalVariables|GetSelectedClassIndex)))))
                (:NewEnumerator1
                  (return (.pawnclass (Utilities|Array|Get(acopy) (Variables|/Game/EyeContact/Blueprints/BP_EyeContactGameInstance.BP_EyeContactGameInstance_C|GetMonsterClasses _asbp_eye_contact_game_instance) (LocalVariables|GetSelectedClassIndex)))))
                (:NewEnumerator2
                  ;[1 1 1] For editor only
                  (switch int (Math|Random|RandomInteger 2)
                    (:Default
                      (Utilities|Array|Add (Variables|/Game/EyeContact/Blueprints/BP_EyeContactGameInstance.BP_EyeContactGameInstance_C|GetHumanPlayerIds _asbp_eye_contact_game_instance) (Variables|/Script/Engine.PlayerState|GetPlayerId (Variables|/Script/Engine.Controller|GetPlayerState _asbp_eye_contact_controller)) :!label _label)
                      (Utilities|Array|Add (Variables|/Game/EyeContact/Blueprints/BP_EyeContactGameInstance.BP_EyeContactGameInstance_C|GetPlayerClassIds _asbp_eye_contact_game_instance) (Utilities|Struct|MakeIntPair (Variables|/Script/Engine.PlayerState|GetPlayerId (Variables|/Script/Engine.Controller|GetPlayerState _asbp_eye_contact_controller)) 0))
                      (return "/Game/EyeContact/Blueprints/BP_HumanDefender.BP_HumanDefender_C"))
                    (:0
                      (Utilities|Array|Add (Variables|/Game/EyeContact/Blueprints/BP_EyeContactGameInstance.BP_EyeContactGameInstance_C|GetMonsterPlayerIds _asbp_eye_contact_game_instance) (Variables|/Script/Engine.PlayerState|GetPlayerId (Variables|/Script/Engine.Controller|GetPlayerState _asbp_eye_contact_controller)))
                      (Utilities|Array|Add (Variables|/Game/EyeContact/Blueprints/BP_EyeContactGameInstance.BP_EyeContactGameInstance_C|GetPlayerClassIds _asbp_eye_contact_game_instance) (Utilities|Struct|MakeIntPair (Variables|/Script/Engine.PlayerState|GetPlayerId (Variables|/Script/Engine.Controller|GetPlayerState _asbp_eye_contact_controller)) 0)))
                    (:1
                      (goto _label))))))
            (:CastFailed
              _)))
        (:CastFailed
          _))
      (return "/Game/EyeContact/Blueprints/BP_MonsterPlayer.BP_MonsterPlayer_C"))))