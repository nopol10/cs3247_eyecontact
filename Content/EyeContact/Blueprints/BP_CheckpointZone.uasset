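; Checkpoint trigger zone for co-op play that records how far the human Killer and Spotter have progressed.
; On the server, overlap by either character activates the zone once, only if its index exceeds the saved one.
; Activation writes the index to the game instance's CoopCheckpoint and prints it.
; OnSpawnHere, not called within this Blueprint, destroys the actors listed in ObjectsToKill.
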(event OnComponentBeginOverlap(Box)
  (params (OverlappedComponent :type Primitive%20Component%20Object%20Reference) (OtherActor :type Actor%20Object%20Reference) (OtherComp :type Primitive%20Component%20Object%20Reference) (OtherBodyIndex :type Integer) (bFromSweep :type Boolean) (SweepResult :type Hit%20Result%20Structure%20%28by%20ref%29))
  (Networking|SwitchHasAuthority
    (:Authority
      (bind _canactivate (CallFunction|CanActivate))
      (if _canactivate
        (Utilities|Casting|CastToBP_CoopHumanKiller OtherActor
          (:then
            _)
          (:CastFailed
            (Utilities|Casting|CastToBP_CoopHumanSpotter OtherActor)))
        (Variables|Default|SetIsActivated true)
        (bind _asbp_eye_contact_game_instance (Utilities|Casting|CastToBP_EyeContactGameInstance (Game|GetGameInstance)))
        (Variables|/Game/EyeContact/Blueprints/BP_EyeContactGameInstance.BP_EyeContactGameInstance_C|SetCoopCheckpoint _asbp_eye_contact_game_instance (Variables|Default|GetCheckpointIndex))
        (Development|PrintString (Utilities|String|Append "Checkpoint " (Utilities|String|ToString(Integer) (Variables|Default|GetCheckpointIndex))))))))

(event EventBeginPlay)

(event Collision|EventActorBeginOverlap
  (params (OtherActor :type Actor%20Object%20Reference)))

(event EventTick
  (params (DeltaSeconds :type Float%20%28single-precision%29)))

(fn ConstructionScript)

(fn CanActivate
  (bind _asbp_eye_contact_game_instance (Utilities|Casting|CastToBP_EyeContactGameInstance (Game|GetGameInstance))
    (:then
      (return (and (not (Variables|Default|GetIsActivated)) (> (Variables|Default|GetCheckpointIndex) (Variables|/Game/EyeContact/Blueprints/BP_EyeContactGameInstance.BP_EyeContactGameInstance_C|GetCoopCheckpoint _asbp_eye_contact_game_instance)))))
    (:CastFailed
      (return false))))

(fn OnSpawnHere
  (for _array_element (Variables|Default|GetObjectsToKill)
    (Actor|DestroyActor _array_element)))