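; BP_EndGoal is the exit zone that lets the human team win when entered.
; Its box overlap runs only on the server and ends the match through EyeContactGameMode.
; An overlapping BP_HumanVIP wins immediately, covering VIP mode.
; Other human players win only when the game mode and player both report holding the goal object; otherwise they get a face message to find the sword.
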(event OnComponentBeginOverlap(Box)
  (params (OverlappedComponent :type Primitive%20Component%20Object%20Reference) (OtherActor :type Actor%20Object%20Reference) (OtherComp :type Primitive%20Component%20Object%20Reference) (OtherBodyIndex :type Integer) (bFromSweep :type Boolean) (SweepResult :type Hit%20Result%20Structure%20%28by%20ref%29))
  (Networking|SwitchHasAuthority
    (:Authority
      (Utilities|Casting|CastToBP_HumanVIP OtherActor
        (:then
          ;[1 1 1] VIP Mode Ending
          (bind _aseye_contact_game_mode (Utilities|Casting|CastToEyeContactGameMode (Game|GetGameMode)))
          (Default|HumansWin _aseye_contact_game_mode))
        (:CastFailed
          (bind _asbp_human_player (Utilities|Casting|CastToBP_HumanPlayer OtherActor))
          (bind _aseye_contact_game_mode_2 (Utilities|Casting|CastToEyeContactGameMode (Game|GetGameMode)))
          (if (and (Variables|/Game/EyeContact/Blueprints/EyeContactGameMode.EyeContactGameMode_C|GetHumansHaveGoal _aseye_contact_game_mode_2) (Variables|/Game/EyeContact/Blueprints/BP_HumanPlayer.BP_HumanPlayer_C|GetHasGoalObject _asbp_human_player))
            (Default|HumansWin _aseye_contact_game_mode_2)
            (else
              (Default|ShowFaceMessagefromServer _asbp_human_player "Find the sword before leaving!" 2.0 13.0))))))))

(event EventBeginPlay)

(event EventActorBeginOverlap
  (params (OtherActor :type Actor%20Object%20Reference)))

(event EventTick
  (params (DeltaSeconds :type Float%20%28single-precision%29)))

(fn ConstructionScript)