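; End goal trigger for co-op mode that wins the match on the server when its box is overlapped.
; BeginPlay offsets the gate upward and creates a dynamic material on BrightWall.
; The first killer or spotter overlap plays a timeline driving gate height and wall Strength, on authority only.
; The game mode's ServerWinCoop call runs on every authority overlap, regardless of actor type or prior activation.
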(event OnComponentBeginOverlap(Box)
  (params (OverlappedComponent :type Primitive%20Component%20Object%20Reference) (OtherActor :type Actor%20Object%20Reference) (OtherComp :type Primitive%20Component%20Object%20Reference) (OtherBodyIndex :type Integer) (bFromSweep :type Boolean) (SweepResult :type Hit%20Result%20Structure%20%28by%20ref%29))
  (Development|PrintString "Hello")
  (Networking|SwitchHasAuthority
    (:Authority
      (Utilities|FlowControl|Sequence
        (:then_0
          (if (not (Variables|Default|GetIsActivated))
            (Utilities|Casting|CastToBP_CoopHumanKiller OtherActor
              (:then
                _)
              (:CastFailed
                (Utilities|Casting|CastToBP_CoopHumanSpotter OtherActor)))
            (Variables|Default|SetIsActivated true)
            (bind _alpha (Timeline|MoveGate PlayFromStart)
              (:Update
                (Transformation|SetActorLocation (Variables|Default|GetGate) (+ (Variables|Default|GetOriginalGatePosition) (* "0, 0,500.000000" _alpha)) false true)
                (Rendering|Material|SetScalarParameterValue (Variables|Default|GetWallDMI) "Strength" _alpha :!class /Script/Engine.MaterialInstanceDynamic)))))
        (:then_1
          (bind _aseye_contact_coop_mode (Utilities|Casting|CastToEyeContactCoopMode (Game|GetGameMode)))
          (Default|ServerWinCoop _aseye_contact_coop_mode (Variables|Default|GetBrightWall)))))))

(event EventBeginPlay
  ;[1 1 1] SetGate
  (Utilities|FlowControl|Sequence
    (:then_0
      (bind _output_get (Variables|Default|SetOriginalGatePosition (Transformation|GetActorLocation (Variables|Default|GetGate))))
      (Transformation|SetActorLocation (Variables|Default|GetGate) (+ _output_get "0.000000, 0,500.000000") false false))
    (:then_1
      (bind _asstatic_mesh_actor (Utilities|Casting|CastToStaticMeshActor (Variables|Default|GetBrightWall)))
      (bind _returnvalue (Rendering|Material|CreateDynamicMaterialInstance (Variables|/Script/Engine.StaticMeshActor|GetStaticMeshComponent _asstatic_mesh_actor) 0 (Utilities|Array|Get(acopy) (Rendering|Material|GetMaterials (Variables|/Script/Engine.StaticMeshActor|GetStaticMeshComponent _asstatic_mesh_actor))) :!class /Script/Engine.PrimitiveComponent))
      (Variables|Default|SetWallDMI _returnvalue))))

(fn ConstructionScript)

(fn OnRepGate)