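; BP_HumanShield is a timed skill actor that follows a linked actor as its shield.
; BeginPlay starts a countdown from Timeout, and Tick reduces it by delta time while moving the shield to the linked actor's location if that actor is valid.
; On expiry it clears the linked actor's IsShielded flag, without a validity check, and destroys itself; this file never sets the flag true.
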(event EventBeginPlay
  (Variables|Default|SetCountdown (Variables|Default|GetTimeout)))

(event Collision|EventActorBeginOverlap
  (params (OtherActor :type Actor%20Object%20Reference)))

(event EventTick
  (params (DeltaSeconds :type Float%20%28single-precision%29))
  (bind _linkedactor (Variables|Default|GetLinkedActor))
  (bind _output_get (Variables|Default|SetCountdown (- (Variables|Default|GetCountdown) DeltaSeconds)))
  (if (<= _output_get 0.0)
    (Variables|/Game/EyeContact/Blueprints/BP_HumanPlayer.BP_HumanPlayer_C|SetIsShielded (Variables|Default|GetLinkedActor) false)
    (Actor|DestroyActor)
    (else
      (Utilities|IsValid _linkedactor
        (:Is%20Valid
          (Transformation|SetActorLocation (Transformation|GetActorLocation _linkedactor) false false))))))

(fn ConstructionScript)