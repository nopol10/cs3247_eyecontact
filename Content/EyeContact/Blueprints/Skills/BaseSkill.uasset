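; BaseSkill is a replicated component base for skills, with a cooldown and a friendly, enemy or everyone target type.
; An indexed activation request calls the empty ActivateSkillActual hook for children to override, then starts the cooldown, which Tick counts down.
; Helpers report cooldown progress, test or branch on target type, and spawn a homing projectile at the owner with a given particle class and target.
; BeginPlay caches the owner's first camera component.
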(event Custom|ActivateSkillWithCheck
  (params (SkillIndex :type Integer))
  (if (== SkillIndex (Variables|Default|GetSkillIndex))
    (if (not (> (Variables|Default|GetCooldownTimer) 0.0))
      (CallFunction|ActivateSkillActual)
      (Variables|Default|SetCooldownTimer (Variables|Default|GetCooldown)))))

(event Custom|SpawnHomingProjectile
  (params (ParticleClass :type Particle%20System%20Object%20Reference) (ActorTarget :type Actor%20Object%20Reference))
  (bind _returnvalue (Game|SpawnActorfromClass "/Game/EyeContact/Blueprints/Projectiles/BP_HomingProjectile.BP_HomingProjectile_C" (Transformation|GetActorTransform (Components|GetOwner)) "Undefined" 0 0))
  (Default|SetParticleClass _returnvalue ParticleClass)
  (Default|SetTarget _returnvalue ActorTarget)
  (Variables|Default|SetProjectile _returnvalue))

(event Custom|ActivateSkillActual)

(event EventBeginPlay
  (Class|ActorComponent|SetIsReplicated true)
  (bind _array_element (Utilities|Array|ForEachLoopwithBreak (Actor|GetComponentsByClass (Components|GetOwner) "/Script/Engine.CameraComponent") :!label _label)
    (:LoopBody
      (Variables|Components|SetPlayerCamera _array_element)
      (goto _label Break))))

(event EventTick
  (params (DeltaSeconds :type Float%20%28single-precision%29))
  (Variables|Default|SetCooldownTimer (Math|Float|Max(Float) (- (Variables|Default|GetCooldownTimer) DeltaSeconds) 0.0)))

(fn IsFriendlySkill
  (if (== (Variables|Default|GetTargetType) 0)
    (return true)
    (else
      (return false))))

(fn IsEnemySkill
  (if (== (Variables|Default|GetTargetType) 1)
    (return true)
    (else
      (return false))))

(fn IsEveryoneSkill
  (if (== (Variables|Default|GetTargetType) 2)
    (return true)
    (else
      (return false))))

(fn GetCooldownPercent
  (return (- 1.0 (/ (Variables|Default|GetCooldownTimer) (Variables|Default|GetCooldown)))))