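; Skill that casts a protective shield onto other human players within an angle of the owning pawn.
; On activation it checks every BP_HumanPlayer and fires a homing spark projectile at each one in the cone, with no team check.
; When a projectile reaches its target, it spawns a BP_HumanShield linked to that player and flags them as shielded.
; A CheckTargetType macro branches friendly, enemy or both but is not called here.
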(event Custom|CastShieldOnAlly
  (params (Ally :type BP%20Human%20Player%20Object%20Reference))
  (CallFunction|SpawnHomingProjectile "/Game/StarterContent/Particles/P_Sparks.P_Sparks" Ally)
  (EventDispatchers|BindEventtoOnReachTarget (Variables|Default|GetProjectile) (delegate Custom|ShieldProjectileReached)))

(event Custom|ShieldProjectileReached
  (params (Target :type Actor%20Object%20Reference))
  (bind _asbp_human_player (Utilities|Casting|CastToBP_HumanPlayer Target))
  (bind _returnvalue (Game|SpawnActorfromClass "/Game/EyeContact/Blueprints/Skills/BP_HumanShield.BP_HumanShield_C" (Transformation|GetActorTransform Target) "Undefined" 0 0))
  (Variables|/Game/EyeContact/Blueprints/Skills/BP_HumanShield.BP_HumanShield_C|SetLinkedActor _returnvalue _asbp_human_player)
  (Variables|/Game/EyeContact/Blueprints/BP_HumanPlayer.BP_HumanPlayer_C|SetIsShielded _asbp_human_player true))

(event EventBeginPlay)

(event EventTick
  (params (DeltaSeconds :type Float%20%28single-precision%29)))

(event EventActivateSkillActual
  (Development|PrintString "Skill cast shield activated")
  (bind _aspawn (Utilities|Casting|CastToPawn (Components|GetOwner)))
  (bind _outactors (Actor|GetAllActorsOfClass "/Game/EyeContact/Blueprints/BP_HumanPlayer.BP_HumanPlayer_C"))
  (bind _array_element (Utilities|Array|ForEachLoopwithBreak _outactors)
    (:LoopBody
      (bind _withinangle (CallFunction|ActorWithinAngle _aspawn _array_element 45.0))
      (if (and (!= _aspawn _array_element) _withinangle)
        (Development|PrintString "Actor within angle")
        (CallFunction|CastShieldonAlly _array_element)))))