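; SkillOutline is a skill Blueprint that triggers an outline effect on every human player in the level.
; On activation it prints a debug string, gathers all BP_HumanPlayer actors and passes each through OutlineEvent to the OutlineHuman function.
; OutlineHuman calls EchoHit on the target with the skill's effect duration, leaving the effect itself to the human player Blueprint.
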(event Custom|OutlineEvent
  (params (HumanTarget :type BP%20Human%20Player%20Object%20Reference))
  (CallFunction|OutlineHuman HumanTarget))

(event EventBeginPlay
  (|CallParentFunction))

(event EventTick
  (params (DeltaSeconds :type Float%20%28single-precision%29))
  (|CallParentFunction 0.0))

(event EventActivateSkillActual
  (Development|PrintString "Skill outline!")
  (bind _outactors (Actor|GetAllActorsOfClass "/Game/EyeContact/Blueprints/BP_HumanPlayer.BP_HumanPlayer_C"))
  (bind _array_element (Utilities|Array|ForEachLoopwithBreak _outactors)
    (:LoopBody
      (CallFunction|OutlineEvent _array_element))))

(fn OutlineHuman
  (params (HumanTarget :type BP%20Human%20Player%20Object%20Reference))
  (Default|EchoHit HumanTarget (Variables|Default|GetSkillEffectDuration))
  (return))