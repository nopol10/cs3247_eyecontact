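; SkillCureBlindness is a skill that clears blindness from other human players near the pawn that owns it.
; On activation it scans every BP_HumanPlayer, skips the owner and sets IsBlind to false on those within CastRange.
; A CheckTargetType branch sorts TargetType into friendly, enemy or both, but activation never uses it, so no team filtering applies.
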(event Custom|CureBlindnessOnAlly
  (params (Ally :type BP%20Human%20Player%20Object%20Reference))
  (Variables|/Game/EyeContact/Blueprints/BP_HumanPlayer.BP_HumanPlayer_C|SetIsBlind Ally false))

(event EventBeginPlay)

(event EventTick
  (params (DeltaSeconds :type Float%20%28single-precision%29)))

(event EventActivateSkillActual
  (Development|PrintString "Skill cure blindness activated")
  (bind _aspawn (Utilities|Casting|CastToPawn (Components|GetOwner)))
  (bind _outactors (Actor|GetAllActorsOfClass "/Game/EyeContact/Blueprints/BP_HumanPlayer.BP_HumanPlayer_C"))
  (bind _array_element (Utilities|Array|ForEachLoopwithBreak _outactors)
    (:LoopBody
      (bind _withindistance (CallFunction|ActorsWithinDistance _array_element _aspawn (Variables|Default|GetCastRange)))
      (if (and (!= _aspawn _array_element) _withindistance)
        (Development|PrintString "Actor within distance")
        (CallFunction|CureBlindnessonAlly _array_element)))))