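; SkillWall is a human player skill that places a temporary BP_CommanderWall in the world.
; Activating it off cooldown toggles build mode, spawning a collisionless preview wall; activating again cancels it.
; Each tick, camera line traces position the preview, dropping downward onto a surface when they hit steep faces or nothing.
; BuildWall swaps the preview for a wall spawned through ServerBuildWall with the effect duration, then starts cooldown.
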(event Custom|ServerBuildWall
  (bind _returnvalue (Game|SpawnActorfromClass "/Game/EyeContact/Blueprints/BP_CommanderWall.BP_CommanderWall_C" (Variables|Default|GetWallTransform) "Undefined" 0 0))
  (Default|BuildWall _returnvalue (Variables|Default|GetSkillEffectDuration))
  (CallFunction|StartCoolDown))

(event Custom|BuildWall
  (bind _wall (Variables|Default|GetWall))
  (Variables|Default|SetIsBuildMode false)
  (if (Utilities|IsValid _wall)
    (Variables|Default|SetWallTransform (Transformation|GetActorTransform _wall))
    (Actor|DestroyActor _wall)
    (CallFunction|ServerBuildWall)))

(event Custom|StartCoolDown
  (Variables|Default|SetCooldownTimer (Variables|Default|GetCooldown)))

(event Custom|OwningClientSkillCheck
  (if (Variables|Default|GetIsBuildMode)
    (Variables|Default|SetIsBuildMode false)
    (if (Utilities|IsValid (Variables|Default|GetWall))
      (Actor|DestroyActor (Variables|Default|GetWall)))
    (elif (not (> (Variables|Default|GetCooldownTimer) 0.0))
      (Variables|Default|SetIsBuildMode true)
      (bind _returnvalue (Game|SpawnActorfromClass "/Game/EyeContact/Blueprints/BP_CommanderWall.BP_CommanderWall_C" (Math|Transform|MakeTransform "0, 0, 0") "Undefined" 0 0))
      (bind _output_get (Variables|Default|SetWall _returnvalue))
      (Default|SetOpacity _output_get false)
      (Collision|SetCollisionEnabled (Variables|/Game/EyeContact/Blueprints/BP_CommanderWall.BP_CommanderWall_C|GetWallMesh _output_get) "NoCollision"))))

(event EventBeginPlay
  (bind _tracetypes (Variables|Default|GetTraceTypes))
  (|CallParentFunction)
  (bind _asbp_human_player (Utilities|Casting|CastToBP_HumanPlayer (Components|GetOwner)))
  (Variables|Default|SetHumanOwner _asbp_human_player)
  (Utilities|Array|Insert _tracetypes "ObjectTypeQuery1")
  (Utilities|Array|Insert _tracetypes "ObjectTypeQuery2" 1)
  (bind _outactors (Actor|GetAllActorsOfClass "/Game/EyeContact/Blueprints/BP_HumanVIP.BP_HumanVIP_C"))
  (if (> (Utilities|Array|Length _outactors) 0)
    (Variables|Default|SetVIP (Utilities|Array|Get(acopy) _outactors))))

(event EventTick
  (params (DeltaSeconds :type Float%20%28single-precision%29))
  (bind _humanowner (Variables|Default|GetHumanOwner))
  (bind _camera (Variables|/Game/EyeContact/Blueprints/BP_HumanPlayer.BP_HumanPlayer_C|GetCamera _humanowner))
  (|CallParentFunction DeltaSeconds)
  (if (Variables|Default|GetIsBuildMode)
    (bind _wallpos (CallFunction|LineCastGetWallPosition (Transformation|GetWorldLocation _camera) (Math|Vector|GetForwardVector _camera)))
    (if (Math|Vector|NotEqual(Vector) _wallpos (Variables|Default|GetInvalidVector) 0.0001)
      (Transformation|SetActorLocation (Variables|Default|GetWall) _wallpos false true))))

(event EventActivateSkillwithCheck
  (params (SkillIndex :type Integer))
  (if (== SkillIndex (Variables|Default|GetSkillIndex))
    (CallFunction|OwningClientSkillCheck)))

(fn LineCastGetWallPosition
  (params (CamLoc :type Vector) (CamForwardVect :type Vector))
  (bind _range (Variables|Default|GetRange))
  (bind _returnvalue (* CamForwardVect _range))
  (bind _returnvalue_2 (+ CamLoc _returnvalue))
  (bind (_outhit _returnvalue_3) (Collision|LineTraceForObjects CamLoc _returnvalue_2 (Variables|Default|GetTraceTypes) false 0 "ForOneFrame"))
  (if _returnvalue_3
    (bind _angle (CallFunction|AngleBetweenTwoVectors "0,0.000000,1.000000" (.ImpactNormal (Collision|BreakHitResult _outhit))))
    (if (> _angle 5e+01)
      (bind (_outhit_2 _returnvalue_4) (Collision|LineTraceForObjects (.Location (Collision|BreakHitResult _outhit)) (+ (.Location (Collision|BreakHitResult _outhit)) (* "0,0.000000,-1.000000" 10000)) (Variables|Default|GetTraceTypes) false 0 "ForOneFrame"))
      (if _returnvalue_4
        (return (.Location (Collision|BreakHitResult _outhit_2)))
        (else
          (return (Variables|Default|GetInvalidVector))))
      (else
        (return (.Location (Collision|BreakHitResult _outhit)))))
    (else
      (bind (_outhit_3 _returnvalue_5) (Collision|LineTraceForObjects _returnvalue_2 (+ _returnvalue_2 (* "0,0.000000,-1.000000" 10000)) (Variables|Default|GetTraceTypes) false 0 "ForOneFrame"))
      (if _returnvalue_5
        (return (.Location (Collision|BreakHitResult _outhit_3)))
        (else
          (return (Variables|Default|GetInvalidVector)))))))