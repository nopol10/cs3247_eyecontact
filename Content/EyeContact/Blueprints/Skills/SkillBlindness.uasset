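; Blindness skill that blinds other human players in front of the pawn that owns it.
; On activation it scans all BP_HumanPlayer actors and picks those other than the owner that pass a 45-degree angle check.
; It fires a fire-particle homing projectile at each one, with the reach-target event bound to call BlindHit using the skill's effect duration.
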(event Custom|BlindEvent
  (params (TargetHuman :type BP%20Human%20Player%20Object%20Reference))
  (CallFunction|SpawnHomingProjectile "/Game/StarterContent/Particles/P_Fire_Projectile.P_Fire_Projectile" TargetHuman)
  (EventDispatchers|BindEventtoOnReachTarget (Variables|Default|GetProjectile) (delegate Custom|BlindHuman)))

(event Custom|BlindHuman
  (params (Target :type Actor%20Object%20Reference))
  (bind _asbp_human_player (Utilities|Casting|CastToBP_HumanPlayer Target))
  (Default|BlindHit _asbp_human_player (Variables|Default|GetSkillEffectDuration)))

(event EventBeginPlay
  (|CallParentFunction))

(event EventTick
  (params (DeltaSeconds :type Float%20%28single-precision%29))
  (|CallParentFunction 0.0))

(event EventActivateSkillActual
  (Development|PrintString "Skill blindness")
  (bind _aspawn (Utilities|Casting|CastToPawn (Components|GetOwner)))
  (bind _outactors (Actor|GetAllActorsOfClass "/Game/EyeContact/Blueprints/BP_HumanPlayer.BP_HumanPlayer_C"))
  (bind _array_element (Utilities|Array|ForEachLoopwithBreak _outactors)
    (:LoopBody
      (bind _withinangle (CallFunction|ActorWithinAngle _aspawn _array_element 45.0))
      (if (and (!= _aspawn _array_element) _withinangle)
        (Development|PrintString "Actor within angle")
        (CallFunction|BlindEvent _array_element)))))