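; SkillRoar is a skill that lets its owning pawn roar at human players it is facing.
; On activation it gets all BP_HumanPlayer actors and keeps those other than itself that pass a narrow ActorWithinAngle check, with no distance test in this graph.
; Each match goes through RoarTargetEvent to RoarTarget, which calls RoarHit on that player with the skill's effect duration.
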(event Custom|RoarTargetEvent
  (params (HumanTarget :type BP%20Human%20Player%20Object%20Reference))
  (CallFunction|RoarTarget HumanTarget))

(event EventBeginPlay
  (|CallParentFunction))

(event EventTick
  (params (DeltaSeconds :type Float%20%28single-precision%29))
  (|CallParentFunction 0.0))

(event EventActivateSkillActual
  (Development|PrintString "Skill roar!")
  (bind _aspawn (Utilities|Casting|CastToPawn (Components|GetOwner)))
  (bind _outactors (Actor|GetAllActorsOfClass "/Game/EyeContact/Blueprints/BP_HumanPlayer.BP_HumanPlayer_C"))
  (bind _array_element (Utilities|Array|ForEachLoopwithBreak _outactors)
    (:LoopBody
      (bind _withinangle (CallFunction|ActorWithinAngle _aspawn _array_element 1e+01))
      (if (and (!= _aspawn _array_element) _withinangle)
        (Development|PrintString "Actor within angle")
        (CallFunction|RoarTargetEvent _array_element)))))

(fn RoarTarget
  (params (HumanTarget :type BP%20Human%20Player%20Object%20Reference))
  (Default|RoarHit HumanTarget (Variables|Default|GetSkillEffectDuration))
  (return))