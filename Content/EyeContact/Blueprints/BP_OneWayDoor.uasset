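; One-way door that toggles open or closed only when the interacting actor overlaps its FrontSide volume.
; Interact flips DoorOpenFront on the authority, and its RepNotify calls OpenFront to animate the change.
; OpenFront plays or reverses a timeline from either end, lerping DoorBody's relative rotation using FrontRotation.
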(event EventBeginPlay)

(event Collision|EventActorBeginOverlap
  (params (OtherActor :type Actor%20Object%20Reference)))

(event EventTick
  (params (DeltaSeconds :type Float%20%28single-precision%29)))

(fn ConstructionScript)

(fn OnRepDoorOpenFront
  (CallFunction|OpenFront))

(event Custom|Open%20Front
  (if (Variables|Default|GetDoorOpenFront)
    (bind _doormovement (Timeline|Timeline_0 ReverseFromEnd)
      (:Update
        (Transformation|SetRelativeRotation (Variables|Default|GetDoorBody) (Math|Rotator|Lerp(Rotator) (Variables|Default|GetFrontRotation) "0, 0, 0" _doormovement) false false)))
    (else
      (Timeline|Timeline_0 PlayFromStart))))

(event EventInteract
  (params (Interactor :type Actor%20Object%20Reference))
  (Networking|SwitchHasAuthority
    (:Authority
      (if (Collision|IsOverlappingActor (Variables|Default|GetFrontSide) Interactor :!class /Script/Engine.PrimitiveComponent)
        (if (Variables|Default|GetDoorOpenFront)
          (Variables|Default|SetDoorOpenFront false)
          (else
            (Variables|Default|SetDoorOpenFront true)))))))