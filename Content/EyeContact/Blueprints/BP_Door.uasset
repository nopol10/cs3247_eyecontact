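; BP_Door is an interactable door that toggles between open and closed.
; The Interact event checks the DoorOpen flag, calls OpenDoor or CloseDoor, then flips the flag.
; Both functions snap the DoorBody component's relative yaw instantly between closed and swung-open angles, with no timeline or interpolation.
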(event EventBeginPlay)

(event EventActorBeginOverlap
  (params (OtherActor :type Actor%20Object%20Reference)))

(event EventTick
  (params (DeltaSeconds :type Float%20%28single-precision%29)))

(event EventInteract
  (params (Interactor :type Actor%20Object%20Reference))
  (if (Variables|Default|GetDoorOpen)
    (CallFunction|CloseDoor)
    (Variables|Default|SetDoorOpen false)
    (else
      (CallFunction|OpenDoor)
      (Variables|Default|SetDoorOpen true))))

(fn ConstructionScript)

(fn OpenDoor
  (Transformation|SetRelativeRotation (Variables|Default|GetDoorBody) "0,80.000000, 0" false false))

(fn CloseDoor
  (Transformation|SetRelativeRotation (Variables|Default|GetDoorBody) "0, 0, 0" false false))