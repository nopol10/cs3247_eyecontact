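; BP_Fader is a utility actor that fades to and from black using a mesh material.
; The construction script creates a dynamic M_Fade instance on its StaticMesh.
; FadeToBlack and FadeFromBlack events drive the Opacity parameter through separate timelines, setting play rate to the inverse of the requested duration.
; FadeToBlack resets opacity to zero on finishing, so it does not hold black.
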(event Custom|Fade%20To%20Black
  (params (Duration :type Float%20%28single-precision%29))
  (Components|Timeline|SetPlayRate (Variables|Default|GetFadeUp) (/ 1.0 Duration))
  (bind _data (Timeline|FadeUp PlayFromStart)
    (:Update
      (Rendering|Material|SetScalarParameterValue (Variables|Default|GetDMI) "Opacity" _data :!class /Script/Engine.MaterialInstanceDynamic))
    (:Finished
      (Rendering|Material|SetScalarParameterValue (Variables|Default|GetDMI) "Opacity" 0.0 :!class /Script/Engine.MaterialInstanceDynamic))))

(event Custom|Fade%20From%20Black
  (params (Duration :type Float%20%28single-precision%29))
  (Components|Timeline|SetPlayRate (Variables|Default|GetFadeDown) (/ 1.0 Duration))
  (bind _data (Timeline|FadeDown PlayFromStart)
    (:Update
      (Rendering|Material|SetScalarParameterValue (Variables|Default|GetDMI) "Opacity" _data :!class /Script/Engine.MaterialInstanceDynamic))))

(event EventBeginPlay)

(event EventActorBeginOverlap
  (params (OtherActor :type Actor%20Object%20Reference)))

(event EventTick
  (params (DeltaSeconds :type Float%20%28single-precision%29)))

(fn ConstructionScript
  (bind _returnvalue (Rendering|Material|CreateDynamicMaterialInstance (Variables|Default|GetStaticMesh) 0 "/Game/EyeContact/Materials/Base_Mat/M_Fade.M_Fade" :!class /Script/Engine.PrimitiveComponent))
  (Variables|Default|SetDMI _returnvalue))