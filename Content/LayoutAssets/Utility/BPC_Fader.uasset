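; BPC_Fader is an actor component that gives its owner screen fade-to-black and fade-from-black calls.
; On BeginPlay it spawns a BP_Fader actor at the owner's transform and stores it.
; Every tick it moves that actor to match the owner's transform instead of attaching it.
; The FadeToBlack and FadeFromBlack events pass their duration through to the spawned fader, which does the actual fading.
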(event Custom|Fade%20To%20Black
  (params (Duration :type Float%20%28single-precision%29))
  (Default|FadetoBlack (Variables|Default|GetFader) Duration))

(event Custom|Fade%20From%20Black
  (params (Duration :type Float%20%28single-precision%29))
  (Default|FadefromBlack (Variables|Default|GetFader) Duration))

(event EventBeginPlay
  (bind _returnvalue (Game|SpawnActorfromClass "/Game/LayoutAssets/Utility/BP_Fader.BP_Fader_C" (Transformation|GetActorTransform (Components|GetOwner)) "Undefined" 0 0))
  (Variables|Default|SetFader _returnvalue))

(event EventTick
  (params (DeltaSeconds :type Float%20%28single-precision%29))
  (Transformation|SetActorTransform (Variables|Default|GetFader) (Transformation|GetActorTransform (Components|GetOwner))))